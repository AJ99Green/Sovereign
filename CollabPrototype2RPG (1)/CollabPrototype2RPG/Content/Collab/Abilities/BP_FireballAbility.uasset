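; Fireball ability that launches a fireball from the player and deals area damage at a target actor's location.
; UseAbility spawns BP_Fireball at the player's capsule, yawed toward the target, and slides it there over a short fixed time with MoveComponentTo.
; A multi-sphere object trace at the target then applies damage to hit WorldDynamic and Pawn actors, using radius and damage from AbilityStats.
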(event `/Game/Collab/Abilities/BPI_Ability.UseAbility`
  (params (SpawnLocation :type "/Game/Collab/AI/Pawns/BaseEnemyPawn Object Reference"))
  (bind _returnvalue (`self.K2_GetActorLocation` SpawnLocation))
  (bind (_abilitystats_hitfx _abilitystats_damage _abilitystats_damageradius) (break `/Game/Collab/Abilities/S_AbilityStats` (`self.AbilityStats`)))
  (bind _returnvalue_2 (`SceneComponent.K2_GetComponentLocation` (`Character.CapsuleComponent` (`GameplayStatics.GetPlayerCharacter` 0))))
  (bind (_returnvalue_roll _returnvalue_pitch _returnvalue_yaw) (`KismetMathLibrary.BreakRotator` (`KismetMathLibrary.FindLookAtRotation` _returnvalue_2 _returnvalue)))
  (bind _returnvalue_3 (`|SpawnActorFromClass` "/Game/Collab/Abilities/BP_Fireball.BP_Fireball_C" (`KismetMathLibrary.MakeTransform` _returnvalue_2 (`KismetMathLibrary.MakeRotator` 0.0 0.0 _returnvalue_yaw)) "Undefined" "OverrideRootScale" null null))
  (`KismetSystemLibrary.MoveComponentTo` (`Actor.RootComponent` _returnvalue_3) _returnvalue (struct) false false 0.5)
  ;[1 1 1] sphere cast & apply damage
  (bind _outhits (`KismetSystemLibrary.SphereTraceMultiForObjects` :`Start` _returnvalue :`End` _returnvalue :`Radius` _abilitystats_damageradius :`ObjectTypes` (`|MakeArray` "ObjectTypeQuery2" "ObjectTypeQuery3" :!type "EObjectTypeQuery Enum") :`DrawTime` 1.0))
  (for _array_element _outhits
    (`GameplayStatics.ApplyDamage` (`.HitActor` (`GameplayStatics.BreakHitResult` _array_element)) _abilitystats_damage)))

(fn `UserConstructionScript`
  (`parent.UserConstructionScript`))