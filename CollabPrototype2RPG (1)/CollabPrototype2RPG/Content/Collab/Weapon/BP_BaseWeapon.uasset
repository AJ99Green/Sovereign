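; BP_BaseWeapon is a weapon actor that deals light or heavy melee-range damage for the player's TopDownCharacter, which it caches on BeginPlay.
; Attack runs a box trace from the weapon along the player's forward vector, ignoring the player.
; It deduplicates hit actors, then applies light or heavy damage from WeaponStats to each.
; The CantAttack guard resets immediately after the damage pass, with no cooldown.
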(event `self.ReceiveBeginPlay`
  (bind _astop_down_character (cast `/Game/Collab/Character/TopDownCharacter` (`GameplayStatics.GetPlayerCharacter` 0)))
  (set `self.PlayerRef` _astop_down_character))

(event `/Game/Collab/Weapon/BPI_WeaponActions.Attack`
  (params (IsLightAttack :type Boolean))
  (bind _temphitactors (`self.TempHitActors`))
  (bind (_weaponstats_lightattackdamage _weaponstats_heavyattackdamage) (break `/Game/Collab/Weapon/S_WeaponStats` (`self.WeaponStats`)))
  (bind _returnvalue (`self.K2_GetActorLocation` self))
  (set `self.IsLightAttack` IsLightAttack)
  (if (not (`self.CantAttack`))
    (set `self.CantAttack` true)
    (bind _outhits (`KismetSystemLibrary.BoxTraceMultiForObjects` _returnvalue (+ _returnvalue (* (`self.GetActorForwardVector` (`self.PlayerRef`)) 100.0)) (80.0 80.0 80.0) (struct) (`|MakeArray` "ObjectTypeQuery3" "ObjectTypeQuery2" :!type "EObjectTypeQuery Enum") false (`|MakeArray` (`self.PlayerRef`) :!type "Actor Object Reference") "None" true (struct :`R` 1.0 :`A` 1.0) (struct :`G` 1.0 :`A` 1.0) 0.5))
    (for _array_element _outhits
      (`KismetArrayLibrary.Array_AddUnique` (`self.TempHitActors`) (`.HitActor` (`GameplayStatics.BreakHitResult` _array_element))))
    (for _array_element_2 _temphitactors
      (if (`self.IsLightAttack`)
        (`GameplayStatics.ApplyDamage` _array_element_2 _weaponstats_lightattackdamage)
        (else
          (`GameplayStatics.ApplyDamage` _array_element_2 _weaponstats_heavyattackdamage))))
    (set `self.CantAttack` false)
    (`KismetArrayLibrary.Array_Clear` _temphitactors)))

(fn `UserConstructionScript`)