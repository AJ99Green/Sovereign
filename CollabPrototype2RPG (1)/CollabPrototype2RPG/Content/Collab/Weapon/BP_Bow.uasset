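; Bow weapon Blueprint that performs light or heavy hitscan attacks for the top-down player character.
; Attack, gated by CantAttack, halts movement, captures the cursor's world position, waits the WeaponStats duration, then line-traces to that point with debug drawing.
; Light attacks damage the hit actor, while heavy damage has no target connected.
; A second equal delay precedes clearing CantAttack, never set here, and restoring hardcoded walk speed.
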(event `/Game/Collab/Weapon/BPI_WeaponActions.Attack`
  (params (IsLightAttack :type Boolean))
  (bind (_weaponstats_lightattackdamage _weaponstats_heavyattackdamage _weaponstats_lightattackduration _weaponstats_heavyattackduration) (break `/Game/Collab/Weapon/S_WeaponStats` (`self.WeaponStats`)))
  (bind (_weaponstats_lightattackdamage_2 _weaponstats_heavyattackdamage_2 _weaponstats_lightattackduration_2 _weaponstats_heavyattackduration_2) (break `/Game/Collab/Weapon/S_WeaponStats` (`self.WeaponStats`)))
  (bind (_weaponstats_lightattackdamage_3 _weaponstats_heavyattackdamage_3) (break `/Game/Collab/Weapon/S_WeaponStats` (`self.WeaponStats`)))
  (set `self.IsLightAttack` IsLightAttack)
  (if (not (`self.CantAttack`))
    (bind _astop_down_character (cast `/Game/Collab/Character/TopDownCharacter` (`GameplayStatics.GetPlayerCharacter` 0)))
    (bind _charactermovement (`Character.CharacterMovement` _astop_down_character))
    (set `CharacterMovementComponent.MaxWalkSpeed` 0.0 _charactermovement)
    (set `self.TempShotLocation` (`SceneComponent.K2_GetComponentLocation` (`/Game/Collab/Character/TopDownCharacter.CursorToWorld` _astop_down_character)))
    (if (`self.IsLightAttack`)
      (`KismetSystemLibrary.PrintString` "bow light attack")
      (`KismetSystemLibrary.Delay` _weaponstats_lightattackduration_2)
      (else
        (`KismetSystemLibrary.PrintString` "bow heavy attack")
        (`KismetSystemLibrary.Delay` _weaponstats_heavyattackduration_2)))
    (bind _outhit (`KismetSystemLibrary.LineTraceSingleForObjects` (`self.K2_GetActorLocation` self) (`self.TempShotLocation`) (`|MakeArray` "ObjectTypeQuery3" "ObjectTypeQuery2" :!type "EObjectTypeQuery Enum") false (`|MakeArray` _astop_down_character :!type "Actor Object Reference") "ForDuration" true (struct :`R` 1.0 :`A` 1.0) (struct :`G` 1.0 :`A` 1.0) 2.0))
    (if (`self.IsLightAttack`)
      (`GameplayStatics.ApplyDamage` (`.HitActor` (`GameplayStatics.BreakHitResult` _outhit)) _weaponstats_lightattackdamage_3)
      (else
        (`GameplayStatics.ApplyDamage` null _weaponstats_heavyattackdamage_3)))
    (if (`self.IsLightAttack`)
      (`KismetSystemLibrary.Delay` _weaponstats_lightattackduration)
      (else
        (`KismetSystemLibrary.Delay` _weaponstats_heavyattackduration)))
    (set `self.CantAttack` false)
    (set `CharacterMovementComponent.MaxWalkSpeed` 600.0 _charactermovement)))

(fn `UserConstructionScript`
  (`parent.UserConstructionScript`))