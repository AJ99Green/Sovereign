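; Gameplay event manager that replaces placed BP_BaseEvent actors with randomly chosen events at BeginPlay.
; SelectEvent spawns a class from EventsAvailable at each placeholder, copies its spawners and blocking radius, then destroys it; chosen classes leave the pool to avoid repeats.
; Defend Point and Boss Enemy events get random navigable positions for their objective or boss spawner within that radius.
; Each event's start notification opens a WB_Event widget showing it.
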(event `self.ReceiveBeginPlay`
  (`self.GetCurrentEventActors`)
  (for _array_element (`self.EventActors`)
    (bind _out_spawnedevent (`self.SelectEvent` _array_element))
    (`KismetArrayLibrary.Array_RemoveItem` (`self.EventsAvailable`) (`GameplayStatics.GetObjectClass` _out_spawnedevent))
    (add `/Game/Collab/Tech/GameplayEvents/BP_BaseEvent.OnEventStarted` _out_spawnedevent (delegate `OnEventStarted`))))

(event `OnEventStarted`
  (params (Event :type "/Game/Collab/Tech/GameplayEvents/BP_BaseEvent Object Reference"))
  (bind _returnvalue (`|CreateWidget` "/Game/Collab/Tech/GameplayEvents/WB_Event.WB_Event_C" (`GameplayStatics.GetPlayerController` 0)))
  (`UserWidget.AddToViewport` _returnvalue 0)
  (`/Game/Collab/Tech/GameplayEvents/WB_Event.SetDisplayedEvent` _returnvalue Event))

(fn `GetCurrentEventActors`
  (`KismetArrayLibrary.Array_Clear` (`self.EventActors`))
  (bind _outactors (`GameplayStatics.GetAllActorsOfClass` "/Game/Collab/Tech/GameplayEvents/BP_BaseEvent.BP_BaseEvent_C"))
  (for _array_element _outactors
    (`KismetArrayLibrary.Array_Add` (`self.EventActors`) _array_element)))

(fn `SelectEvent`
  (params (EventToReplace :type "/Game/Collab/Tech/GameplayEvents/BP_BaseEvent Object Reference"))
  (returns (Out_SpawnedEvent :type "/Game/Collab/Tech/GameplayEvents/BP_BaseEvent Object Reference"))
  (locals (ChosenEvent :type "/Game/Collab/Tech/GameplayEvents/BP_BaseEvent Class Reference") (SpawnedEvent :type "/Game/Collab/Tech/GameplayEvents/BP_BaseEvent Object Reference"))
  (bind _blockingradius (`/Game/Collab/Tech/GameplayEvents/BP_BaseEvent.BlockingRadius` EventToReplace))
  (bind _eventsavailable (`self.EventsAvailable`))
  (bind _eventactors (`self.EventActors`))
  (`|ExecutionSequence`
    (:`then_0`
      (bind _output_get (set `local.ChosenEvent` (`|GetArrayItem` _eventsavailable (`KismetMathLibrary.RandomIntegerInRange` 0 (`KismetArrayLibrary.Array_LastIndex` _eventsavailable)))))
      (bind _returnvalue (`|SpawnActorFromClass` _output_get (`KismetMathLibrary.MakeTransform` (`self.K2_GetActorLocation` EventToReplace)) "Undefined" "OverrideRootScale" null "NewEnumerator0" (0.0 0.0 0.0) 0.0 500.0 null))
      (set `local.SpawnedEvent` _returnvalue)
      (set `/Game/Collab/Tech/GameplayEvents/BP_BaseEvent.AssociatedSpawners` (`/Game/Collab/Tech/GameplayEvents/BP_BaseEvent.AssociatedSpawners` EventToReplace) _returnvalue)
      (set `/Game/Collab/Tech/GameplayEvents/BP_BaseEvent.BlockingRadius` _blockingradius _returnvalue)
      (bind (_bactive _eventdata _debugdrawtimer _bdrawdebugs _associatedspawners _blockingradius_2 _eventtype) (defaults `Object` _output_get))
      (set `/Game/Collab/Tech/GameplayEvents/BP_BaseEvent.EventType` _eventtype _returnvalue)
      (switch `/Game/Collab/Tech/GameplayEvents/E_EventType` _eventtype
        (:`NewEnumerator0`
          (bind _asbp_defend_point_event (cast `/Game/Collab/Tech/GameplayEvents/BP_DefendPointEvent` _returnvalue))
          (bind _randomlocation (`NavigationSystemV1.K2_GetRandomLocationInNavigableRadius` (`self.K2_GetActorLocation` _returnvalue) (- _blockingradius 150.0) null null))
          (set `/Game/Collab/Tech/GameplayEvents/BP_DefendPointEvent.PointToDefend` _randomlocation _asbp_defend_point_event))
        (:`NewEnumerator1`
          (bind _asbp_mini_boss_event (cast `/Game/Collab/Tech/GameplayEvents/BP_MiniBossEvent` _returnvalue))
          (`/Game/Collab/Tech/GameplayEvents/BP_MiniBossEvent.InitialiseSpawners` _asbp_mini_boss_event)
          (bind _bossspawner (`/Game/Collab/Tech/GameplayEvents/BP_MiniBossEvent.BossSpawner` _asbp_mini_boss_event))
          (`/Engine/EditorBlueprintResources/StandardMacros.IsValid` _bossspawner
            (:`Is Valid`
              (`self.K2_SetActorLocation` _bossspawner _randomlocation false false))))
        (:`NewEnumerator2`
          (cast `/Game/Collab/Tech/GameplayEvents/HelpAllyEvent/BP_HelpAlly` _returnvalue))
        (:`NewEnumerator3`
          (cast `/Game/Collab/Tech/GameplayEvents/BP_GoblinChestEvent` _returnvalue))))
    (:`then_1`
      (`KismetArrayLibrary.Array_RemoveItem` _eventactors EventToReplace)
      (`KismetArrayLibrary.Array_Add` _eventactors (`local.SpawnedEvent`))
      (`self.K2_DestroyActor` EventToReplace)
      (return (`local.SpawnedEvent`)))))

(fn `UserConstructionScript`
  (`self.GetCurrentEventActors`))