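; Gameplay event in which a goblin must survive enemy waves while a chest unlock timer counts up to completion.
; Activation starts two looping timers: one advances unlock progress each second, the other randomly triggers associated spawners.
; Enemy pawns overlapping the goblin's collision cost it fixed health, and depletion fails the event and destroys the goblin component.
; Completion or failure stops spawning, but the unlock timer is never cleared.
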(event `self.ReceiveBeginPlay`
  (`parent.ReceiveBeginPlay`)
  (add `self.OnEventFailed` (`|CreateDelegate` :!event `Failed`))
  (add `self.OnEventComplete` (`|CreateDelegate` :!event `Complete`)))

(event `/Game/Collab/Tech/GameplayEvents/BPI_EventInteraction.ActivateEvent`
  (`parent.ActivateEvent`)
  (if (not (`self.bActive`))
    (set `self.bActive` true)
    (bind _returnvalue (`KismetSystemLibrary.K2_SetTimerDelegate` (delegate `GoblinUnlockTimer`) 1.0 true))
    (set `self.UnlockTimerHandle` _returnvalue)
    (bind _returnvalue_2 (`KismetSystemLibrary.K2_SetTimerDelegate` (delegate `EnemySpawn`) (`self.EnemySpawnFrequency`) true))
    (set `self.EnemySpawningHandle` _returnvalue_2)))

(event `EnemySpawn`
  (for (_array_element _array_index) (`self.AssociatedSpawners`)
    (if (`KismetMathLibrary.RandomBoolWithWeight` 0.5)
      (`/Game/Collab/Tech/AISpawner/BP_EnemySpawnPoint.SpawnEnemy` _array_element (0.0 0.0 0.0)))))

(event `GoblinUnlockTimer`
  (bind _unlockpercentage (`self.UnlockPercentage`))
  (if (< (+ _unlockpercentage 1.0) (`self.TimeToUnlock`))
    (`/Engine/EditorBlueprintResources/StandardMacros.IncrementFloat` _unlockpercentage)
    (else
      (`self.OnEventComplete` self)
      (`KismetSystemLibrary.PrintString` "complete")
      (`KismetSystemLibrary.K2_ClearAndInvalidateTimerHandle` (`self.EnemySpawningHandle`)))))

(event `self.GoblinAttackCollision.OnComponentBeginOverlap`
  (params (OverlappedComponent :type "PrimitiveComponent Object Reference") (OtherActor :type "Actor Object Reference") (OtherComp :type "PrimitiveComponent Object Reference") (OtherBodyIndex :type Integer) (bFromSweep :type Boolean) (SweepResult :type "HitResult Structure (by ref)"))
  (bind _returnvalue (- (`self.GoblinCurrentHealth`) 25.0))
  (if (`KismetMathLibrary.ClassIsChildOf` (`GameplayStatics.GetObjectClass` OtherActor) "/Game/Collab/Tech/AI/Pawns/BaseEnemyPawn.BaseEnemyPawn_C")
    (if (> _returnvalue 0.0)
      (set `self.GoblinCurrentHealth` _returnvalue)
      (else
        (`self.OnEventFailed` self)))))

(event `Failed` :!signature `self.OnEventFailed`
  (params (Event :type "/Game/Collab/Tech/GameplayEvents/BP_BaseEvent Object Reference"))
  (`KismetSystemLibrary.PrintString` "goblin ded :(")
  (`ActorComponent.K2_DestroyComponent` (`self.Goblin`))
  (`KismetSystemLibrary.K2_ClearAndInvalidateTimerHandle` (`self.EnemySpawningHandle`)))

(event `Complete` :!signature `self.OnEventComplete`
  (params (Event :type "/Game/Collab/Tech/GameplayEvents/BP_BaseEvent Object Reference"))
  (set `self.bActive` false))

(fn `UserConstructionScript`
  (`parent.UserConstructionScript`))