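; Gameplay event where the player defends a point against timed waves of enemies.
; On activation, a looping timer spawns waves from associated spawners up to a set count, sending each enemy's AI to a random navigable point in the defend radius.
; A fast polling timer sphere-checks for the player, swapping capture timers that raise enemy capture while they are away and lower it while present.
; Reaching the timeout deactivates the event; an editor debug circle shows the radius.
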(event `/Game/Collab/Tech/GameplayEvents/BPI_EventInteraction.ActivateEvent`
  ;[1 1 1] wave spawning logic
  (`parent.ActivateEvent`)
  (`self.Init`))

(event `self.ReceiveBeginPlay`
  ;[1 1 1] wave spawning logic
  (`parent.ReceiveBeginPlay`))

(event `SpawnWave`
  ;[1 1 1] wave spawning logic
  (`self.OnWaveSpawned` self)
  (for _array_element (`self.AssociatedSpawners`)
    (bind _spawnedactor (`/Game/Collab/Tech/AISpawner/BP_EnemySpawnPoint.SpawnEnemy` _array_element))
    ;;[1 1 1] move the spawned enemy towards the defend point
    (bind _asbase_enemy_controller (cast `/Game/Collab/Tech/AI/Controllers/BaseEnemyController` (`AIBlueprintHelperLibrary.GetAIController` _spawnedactor)))
    (`/Game/Collab/Tech/AI/Controllers/BaseEnemyController.Init` _asbase_enemy_controller)
    (`|AIMoveTo` _spawnedactor (`NavigationSystemV1.K2_GetRandomLocationInNavigableRadius` (`KismetMathLibrary.TransformLocation` (`self.GetTransform`) (`self.PointToDefend`)) (`self.PointRadius`) null null) null)))

(event `Init`
  ;[1 1 1] wave spawning logic
  (`KismetSystemLibrary.PrintString` "init")
  (bind _returnvalue (`KismetSystemLibrary.K2_SetTimerDelegate` (delegate `WaveLoop`) (`self.TimeBetweenWaves`) true))
  (set `self.WaveTimerHandle` _returnvalue)
  (`self.SpawnWave`)
  (`KismetSystemLibrary.K2_SetTimerDelegate` (delegate `PlayerInDefendPointTest`) 0.01 true))

(event `WaveLoop`
  ;[1 1 1] wave spawning logic
  (if (<= (+ (`self.CurrentWave`) 1) (`self.NumberOfWaves`))
    (`/Engine/EditorBlueprintResources/StandardMacros.IncrementInt` (`self.CurrentWave`)
      (:`  `
        (`self.SpawnWave`)))))

(event `PlayerInDefendPointTest`
  (bind _capturetimerhandle (`self.CaptureTimerHandle`))
  (bind _capturetimerhandle_2 (`self.CaptureTimerHandle`))
  ;[1 1 1] defending point logic
  (if (`self.IsPlayerInDefendRadius`)
    (if (`KismetSystemLibrary.K2_IsTimerActiveHandle` _capturetimerhandle_2)
      (`KismetSystemLibrary.K2_ClearAndInvalidateTimerHandle` _capturetimerhandle_2)
      (bind _returnvalue (`KismetSystemLibrary.K2_SetTimerDelegate` (delegate `EnemyCaptureDecrease`) 0.01 true))
      (set `self.CaptureTimerHandle` _returnvalue))
    (else
      (if (`KismetSystemLibrary.K2_IsTimerActiveHandle` _capturetimerhandle)
        (`KismetSystemLibrary.K2_ClearAndInvalidateTimerHandle` _capturetimerhandle))
      (bind _returnvalue_2 (`KismetSystemLibrary.K2_SetTimerDelegate` (delegate `EnemyCaptureIncrease`) 0.01 true))
      (set `self.CaptureTimerHandle` _returnvalue_2))))

(event `EnemyCaptureIncrease`
  ;[1 1 1] defending point logic
  (set `self.EnemyCapturePercentage` (+ (`self.EnemyCapturePercentage`) 0.01))
  (if (>= (`self.EnemyCapturePercentage`) (`self.DefendPointTimeout`))
    (set `self.bActive` false)))

(event `EnemyCaptureDecrease`
  ;[1 1 1] defending point logic
  (set `self.EnemyCapturePercentage` (`KismetMathLibrary.FClamp` (- (`self.EnemyCapturePercentage`) 0.01))))

(event `self.Editor_DrawDebugs`
  (`parent.Editor_DrawDebugs`)
  (`KismetSystemLibrary.DrawDebugCircle` (`KismetMathLibrary.TransformLocation` (`self.GetTransform`) (`self.PointToDefend`)) (`self.PointRadius`) 32 (struct :`R` 0.117607 :`G` 1.0 :`A` 1.0) 0.1 10.0 (1.0 0.0 0.0) (0.0 1.0 0.0)))

(fn `IsPlayerInDefendRadius`
  (returns (bResult :type Boolean))
  (bind _outactors (`KismetSystemLibrary.SphereOverlapActors` (`KismetMathLibrary.TransformLocation` (`self.GetTransform`) (`self.PointToDefend`)) (`self.PointRadius`) (`|MakeArray` "ObjectTypeQuery3" :!type "EObjectTypeQuery Enum")))
  (for _array_element _outactors
    (if (== _array_element (`GameplayStatics.GetPlayerPawn` 0))
      (return true)))
  (return false))

(fn `UserConstructionScript`
  (`parent.UserConstructionScript`))