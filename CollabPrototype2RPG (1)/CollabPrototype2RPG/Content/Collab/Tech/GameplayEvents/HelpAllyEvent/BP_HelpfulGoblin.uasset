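; BP_HelpfulGoblin is a goblin actor in the HelpAllyEvent gameplay event that stays ready to be activated and revealed.
; Activate sets its Active flag and unhides the actor, while cursor hover selects and deselects it through BPAVisualSelection for visual feedback.
; Its InteractCollisionCheck overlap tests for the player pawn but performs no action yet.
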(event `Activate`
  (set `self.bActive` true)
  (`self.SetActorHiddenInGame` false))

(event `self.ReceiveActorBeginCursorOver`
  (`/Game/Collab/Tech/SelectableObject/BPA_VisualSelection.Select` (`self.BPA_VisualSelection`) 5))

(event `self.ReceiveActorEndCursorOver`
  (`/Game/Collab/Tech/SelectableObject/BPA_VisualSelection.Deselect` (`self.BPA_VisualSelection`)))

(event `self.InteractCollisionCheck.OnComponentBeginOverlap`
  (params (OverlappedComponent :type "PrimitiveComponent Object Reference") (OtherActor :type "Actor Object Reference") (OtherComp :type "PrimitiveComponent Object Reference") (OtherBodyIndex :type Integer) (bFromSweep :type Boolean) (SweepResult :type "HitResult Structure (by ref)"))
  (if (== OtherActor (`GameplayStatics.GetPlayerPawn` 0))
    _))

(fn `UserConstructionScript`)