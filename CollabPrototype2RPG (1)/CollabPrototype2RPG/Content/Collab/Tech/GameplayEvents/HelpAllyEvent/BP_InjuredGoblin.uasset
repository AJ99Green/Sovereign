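; BP_InjuredGoblin is an injured goblin actor for a help-ally event that receives a potion from the player.
; Cursor hover toggles a selection highlight, and a range overlap shows prompt text and enables click-to-interact on its sphere.
; Interacting once sets GivenPotion, fires OnGivenPotion and removes one potion from the player's inventory.
; The potion check gates nothing, and the no-potion message is disconnected.
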(event `self.ReceiveActorEndCursorOver`
  (`/Game/Collab/Tech/SelectableObject/BPA_VisualSelection.Deselect` (`self.BPA_VisualSelection`)))

(event `self.ReceiveActorBeginCursorOver`
  (`/Game/Collab/Tech/SelectableObject/BPA_VisualSelection.Select` (`self.BPA_VisualSelection`) 0))

(event `Interact`
  (if (not (`self.bGivenPotion`))
    (bind _astop_down_character (cast `/Game/Collab/Tech/Character/TopDownCharacter` (`GameplayStatics.GetPlayerPawn` 0)))
    (if (`/Game/Collab/Tech/Inventory/BP_EntityInventory.IsItemInInventory` :`self` (`/Game/Collab/Tech/Character/TopDownCharacter.BP_EntityInventory` _astop_down_character) :`ItemID` 2)
      _
      (else
        _))
    (`KismetSystemLibrary.PrintString` "given potion")
    (set `self.bGivenPotion` true)
    (`self.OnGivenPotion`)
    (message `/Game/Collab/Tech/Inventory/BPI_InventoryInteraction.RemoveItem` (`/Game/Collab/Tech/Character/TopDownCharacter.BP_EntityInventory` (cast `/Game/Collab/Tech/Character/TopDownCharacter` (`GameplayStatics.GetPlayerPawn` 0) :!pure true)) 2 1 (struct))))

(event `self.Sphere.OnClicked`
  (params (TouchedComponent :type "PrimitiveComponent Object Reference") (ButtonPressed :type "Key Structure"))
  (if (`self.bRangeCheck`)
    (`self.Interact`)))

(event `self.RangeCheck.OnComponentBeginOverlap`
  (params (OverlappedComponent :type "PrimitiveComponent Object Reference") (OtherActor :type "Actor Object Reference") (OtherComp :type "PrimitiveComponent Object Reference") (OtherBodyIndex :type Integer) (bFromSweep :type Boolean) (SweepResult :type "HitResult Structure (by ref)"))
  (if (== OtherActor (`GameplayStatics.GetPlayerPawn` 0))
    (set `self.bRangeCheck` true)
    (`SceneComponent.SetVisibility` (`self.TextRender`) true false)))

(event `self.RangeCheck.OnComponentEndOverlap`
  (params (OverlappedComponent :type "PrimitiveComponent Object Reference") (OtherActor :type "Actor Object Reference") (OtherComp :type "PrimitiveComponent Object Reference") (OtherBodyIndex :type Integer))
  (if (== (`GameplayStatics.GetPlayerPawn` 0) OtherActor)
    (set `self.bRangeCheck` false)
    (`SceneComponent.SetVisibility` (`self.TextRender`) false false)))

(fn `UserConstructionScript`)