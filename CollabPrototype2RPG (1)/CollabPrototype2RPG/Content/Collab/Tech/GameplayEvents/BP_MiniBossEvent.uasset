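; Gameplay event for a mini-boss encounter, built on a parent event class.
; On activation it spawns the boss and its minions from their spawners, then reports completion when the boss dies; minion deaths do nothing.
; InitialiseSpawners picks a random associated spawner for the boss and assigns the rest to minions, but its call in the event graph is disconnected.
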(event `self.ReceiveBeginPlay`
  (`parent.ReceiveBeginPlay`))

(event `SpawnBoss`
  (bind _bossspawner (`self.BossSpawner`))
  (`/Game/Collab/Tech/AISpawner/BP_EnemySpawnPoint.SpawnEnemy` _bossspawner)
  (add `/Game/Collab/Tech/AISpawner/BP_EnemySpawnPoint.OnSpawnedEnemyDied` _bossspawner (delegate `OnBossDead`))
  (for _array_element (`self.BossMinionSpawners`)
    (`/Game/Collab/Tech/AISpawner/BP_EnemySpawnPoint.SpawnEnemy` _array_element)
    (add `/Game/Collab/Tech/AISpawner/BP_EnemySpawnPoint.OnSpawnedEnemyDied` _array_element (delegate `OnMinionDied`))))

(event `/Game/Collab/Tech/GameplayEvents/BPI_EventInteraction.ActivateEvent`
  (`parent.ActivateEvent`)
  (`self.SpawnBoss`)
  (set `self.bActive` true))

(event `OnBossDead`
  (params (NewParam :type "/Game/Collab/Tech/AISpawner/BP_EnemySpawnPoint Object Reference"))
  (set `self.bActive` false)
  (`self.OnEventComplete` self))

(event `OnMinionDied`
  (params (SpawnPoint :type "/Game/Collab/Tech/AISpawner/BP_EnemySpawnPoint Object Reference")))

(fn `InitialiseSpawners`
  (bind _associatedspawners (`self.AssociatedSpawners`))
  (bind _output_get (set `self.BossSpawner` (`|GetArrayItem` _associatedspawners (`KismetMathLibrary.RandomIntegerInRange` 0 (`KismetArrayLibrary.Array_LastIndex` _associatedspawners)))))
  (for _array_element (`self.AssociatedSpawners`)
    (if (!= _array_element _output_get)
      (`KismetArrayLibrary.Array_Add` (`self.BossMinionSpawners`) _array_element))))

(fn `UserConstructionScript`
  (`parent.UserConstructionScript`))