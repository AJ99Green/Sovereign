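; Shopkeeper actor that highlights on hover and, when clicked with the player in range, opens a merchant dialogue.
; Opening stops player movement, blends the view to the shop's camera and pauses the game after the blend.
; Closing the dialogue restores the previous view target, re-enables the top-down controller and unpauses.
; A separate OpenShopWidget event, not called here, creates the shop UI and disables click movement.
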(event `self.InRangeCheck.OnComponentBeginOverlap`
  (params (OverlappedComponent :type "PrimitiveComponent Object Reference") (OtherActor :type "Actor Object Reference") (OtherComp :type "PrimitiveComponent Object Reference") (OtherBodyIndex :type Integer) (bFromSweep :type Boolean) (SweepResult :type "HitResult Structure (by ref)"))
  ;[1 1 1] Player is now in range of the shop
  (if (== OtherActor (`GameplayStatics.GetPlayerCharacter` 0))
    (set `self.InRange?` true)))

(event `self.InRangeCheck.OnComponentEndOverlap`
  (params (OverlappedComponent :type "PrimitiveComponent Object Reference") (OtherActor :type "Actor Object Reference") (OtherComp :type "PrimitiveComponent Object Reference") (OtherBodyIndex :type Integer))
  ;[1 1 1] Player is no longer in range of shop
  (if (== OtherActor (`GameplayStatics.GetPlayerCharacter` 0))
    (set `self.InRange?` false)))

(event `self.MouseCollision.OnBeginCursorOver`
  (params (TouchedComponent :type "PrimitiveComponent Object Reference"))
  ;[1 1 1] Highlight shopkeeper if the shop isn't open, only when the shop isn't open so it doesn't get highlighted when it is
  (if (not (`self.IsShopOpen`))
    (`/Game/Collab/Tech/SelectableObject/BPI_Selectable.Select` (`self.BPA_VisualSelection`) (`self.ShopHighlightValue`))))

(event `self.MouseCollision.OnEndCursorOver`
  (params (TouchedComponent :type "PrimitiveComponent Object Reference"))
  ;[1 1 1] Unhighlight shopkeeper if the shop isn't open, only when the shop isn't open as it can't be highlighted when it's open
  (if (not (`self.IsShopOpen`))
    (`/Game/Collab/Tech/SelectableObject/BPA_VisualSelection.Deselect` (`self.BPA_VisualSelection`))))

(event `OpenShopWidget`
  ;[1 1 1] Create shop widget, init it and add it to screen
  (bind _returnvalue (`|CreateWidget` "/Game/Collab/Tech/Shop/WB_Shop.WB_Shop_C"))
  (bind _output_get (set `self.ShopUIRef` _returnvalue))
  (`/Game/Collab/Tech/Shop/WB_Shop.Init` _output_get self)
  (`UserWidget.AddToViewport` (`self.ShopUIRef`) 0)
  ;[1 1 1] Temporarily disable click movement so player doesn't move when in shop
  (bind _astop_down_controller (cast `/Game/Collab/Tech/Character/TopDownController` (`GameplayStatics.GetPlayerController` 0)))
  (`/Game/Collab/Tech/Character/TopDownController.Disable` _astop_down_controller))

(event `self.MouseCollision.OnClicked`
  (params (TouchedComponent :type "PrimitiveComponent Object Reference") (ButtonPressed :type "Key Structure"))
  ;[1 1 1] When shopkeeper is clicked check to see if player is in range, if they are then open the shop and pause the game, delay before pause for camera transition
  (if (`self.InRange?`)
    (`self.OpenShop`)
    (`KismetSystemLibrary.Delay` 0.6)
    (`GameplayStatics.SetGamePaused` true)))

(event `OpenShop`
  ;[1 1 1] Checks to see if already open, if not then...
  (if (not (`self.IsShopOpen`))
    ;[1 1 1] Shop is now open
    (set `self.IsShopOpen` true)
    ;[1 1 1] Unhighlight to make sure shopkeep is unhighlighted
    (`/Game/Collab/Tech/SelectableObject/BPA_VisualSelection.Deselect` (`self.BPA_VisualSelection`))
    ;[1 1 1] Save current camera target for switching back
    (set `self.CameraTargetRef` (`Controller.GetViewTarget` (`GameplayStatics.GetPlayerController` 0)))
    (bind _astop_down_character (cast `/Game/Collab/Tech/Character/TopDownCharacter` (`GameplayStatics.GetPlayerPawn` 0)))
    (`/Game/Collab/Tech/Character/TopDownCharacter.TogglePlayerMovement` _astop_down_character false)
    ;[1 1 1] Change camera view to shopkeeper camera, blends over 0.5 seconds
    (`PlayerController.SetViewTargetWithBlend` (`GameplayStatics.GetPlayerController` 0) self 0.5 "VTBlend_Linear" 0.0 false)
    (bind _dialoguewidget (message `/Game/Collab/Tech/Character/GameMode/BPI_DialogueManagement.StartDialogueTree` (`GameplayStatics.GetGameMode`) "/Game/Collab/Tech/Character/GameMode/DT_Merchant.DT_Merchant"))
    (add `/Game/Collab/Tech/UI/Dialogue/WB_PlayerDialogue.OnDialogueClosed` _dialoguewidget (delegate `CloseShop`))))

(event `CloseShop`
  ;[1 1 1] Shop is now closed
  (set `self.IsShopOpen` false)
  ;[1 1 1] Switch back to normal camera target
  (`PlayerController.SetViewTargetWithBlend` (`GameplayStatics.GetPlayerController` 0) (`self.CameraTargetRef`) 0.5 "VTBlend_Linear" 0.0 false)
  ;[1 1 1] Re enable point and click movement
  (bind _astop_down_controller (cast `/Game/Collab/Tech/Character/TopDownController` (`GameplayStatics.GetPlayerController` 0)))
  (`/Game/Collab/Tech/Character/TopDownController.Enable` _astop_down_controller)
  ;[1 1 1] Unpause
  (`GameplayStatics.SetGamePaused` false)
  (message `/Game/Collab/Tech/Character/GameMode/BPI_DialogueManagement.CloseDialogueTree` (`GameplayStatics.GetGameMode`)))

(fn `UserConstructionScript`)