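; Tavern character-switch actor that poses as an idle Warrior or Paladin, shown only if the game instance reports that character unlocked.
; Clicking it while the player is in range opens a confirmation dialogue; cursor hover toggles a highlight.
; CharacterSwitch saves player data to the game instance, destroys the player and has the game mode spawn the displayed character in place.
; The actor then takes on the previous character's type, updating mesh, animation and position.
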(event `Disable`
  (`self.SetActorHiddenInGame` true)
  (set `self.bActive` false))

(event `Enable`
  (`self.SetActorHiddenInGame` false)
  (set `self.bActive` true))

(event `self.ReceiveBeginPlay`
  (`self.UpdateCharacter`)
  (bind _bresult (message `/Game/Collab/Tech/GameInstance/BPI_GameInstance.GetIsCharacterUnlocked` (`GameplayStatics.GetGameInstance`) (`self.Character`)))
  (if _bresult
    (`self.Enable`)
    (else
      (`self.Disable`))))

(event `Init`
  ;[1 1 1] Init
  (bind _astop_down_character (cast `/Game/Collab/Tech/Character/TopDownCharacter` (`GameplayStatics.GetPlayerCharacter` 0)))
  (set `self.PlayerRef` _astop_down_character)
  (bind _asgm_default (cast `/Game/Collab/Tech/Character/GameMode/GM_Default` (`GameplayStatics.GetGameMode`)))
  (set `self.GamemodeRef` _asgm_default)
  (bind _asbp_game_instance (cast `/Game/Collab/Tech/GameInstance/BP_GameInstance` (`GameplayStatics.GetGameInstance`)))
  (set `self.GameInstance` _asbp_game_instance))

(event `self.InRangeCheck.OnComponentBeginOverlap`
  (params (OverlappedComponent :type "PrimitiveComponent Object Reference") (OtherActor :type "Actor Object Reference") (OtherComp :type "PrimitiveComponent Object Reference") (OtherBodyIndex :type Integer) (bFromSweep :type Boolean) (SweepResult :type "HitResult Structure (by ref)"))
  ;[1 1 1] Player is now in range of character switch
  (if (== OtherActor (`GameplayStatics.GetPlayerCharacter` 0))
    (set `self.InRange?` true)
    (`/Engine/EditorBlueprintResources/StandardMacros.DoOnce` false
      (:`Completed`
        (`self.Init`)))))

(event `self.InRangeCheck.OnComponentEndOverlap`
  (params (OverlappedComponent :type "PrimitiveComponent Object Reference") (OtherActor :type "Actor Object Reference") (OtherComp :type "PrimitiveComponent Object Reference") (OtherBodyIndex :type Integer))
  ;[1 1 1] Player is no longer in range of character switch
  (if (== OtherActor (`GameplayStatics.GetPlayerCharacter` 0))
    (set `self.InRange?` false)))

(event `self.MouseCollision.OnBeginCursorOver`
  (params (TouchedComponent :type "PrimitiveComponent Object Reference"))
  ;[1 1 1] Highlight
  (message `/Game/Collab/Tech/SelectableObject/BPI_Selectable.Select` (`self.BPA_VisualSelection`) (`self.HighlightValue`)))

(event `self.MouseCollision.OnEndCursorOver`
  (params (TouchedComponent :type "PrimitiveComponent Object Reference"))
  ;[1 1 1] Highlight
  (message `/Game/Collab/Tech/SelectableObject/BPI_Selectable.Deselect` (`self.BPA_VisualSelection`)))

(event `self.MouseCollision.OnClicked`
  (params (TouchedComponent :type "PrimitiveComponent Object Reference") (ButtonPressed :type "Key Structure"))
  ;[1 1 1] On Clicked, confirmation/diaglouge widget to confirm switch
  (if (`self.InRange?`)
    ;;[1 1 1] Confirmation Widget
    (bind _returnvalue (`|CreateWidget` "/Game/Collab/Tech/CharacterSwitch/WB_CharacterSelectDialogue.WB_CharacterSelectDialogue_C"))
    (bind _output_get (set `self.CharacterSwitchUIRef` _returnvalue))
    (`UserWidget.AddToViewport` _output_get 0)
    (`/Game/Collab/Tech/CharacterSwitch/WB_CharacterSelectDialogue.Init` _output_get self)))

(event `CharacterSwitch`
  ;[1 1 1] Character switch
  (if (`self.bActive`)
    (`PlayerCameraManager.StartCameraFade` :`self` (`GameplayStatics.GetPlayerCameraManager` 0) :`FromAlpha` 2.0 :`Duration` 5.0 :`bShouldFadeAudio` true)
    ;;[1 1 1] Save current character stats to game instance
    (bind (_charactertype _characterstats _inventory_items _playerabilities) (`/Game/Collab/Tech/Character/TopDownCharacter.GetCharacterData` (`self.PlayerRef`)))
    (`/Game/Collab/Tech/GameInstance/BP_GameInstance.SetSavedCharacter` (`self.GameInstance`) _charactertype _characterstats _inventory_items _playerabilities)
    ;;[1 1 1] Save current character type for what character to switch
    (set `self.TempCharacter` (`/Game/Collab/Tech/Character/TopDownCharacter.CharacterType` (`self.PlayerRef`)))
    ;;[1 1 1] Save character transform
    (set `self.CharacterTransform` (`self.GetTransform` (`self.PlayerRef`)))
    ;;[1 1 1] Destroy current character
    (`self.K2_DestroyActor` (`/Game/Collab/Tech/Character/TopDownCharacter.CurrentWeapon` (`self.PlayerRef`)))
    (`self.K2_DestroyActor` (`self.PlayerRef`))
    ;;[1 1 1] Spawn new character
    (`/Game/Collab/Tech/Character/GameMode/GM_Default.SpawnCharacter` (`self.GamemodeRef`) (`self.Character`) (`self.CharacterTransform`))
    (set `self.Character` (`self.TempCharacter`))
    (`self.UpdateCharacter`)
    (bind _astop_down_character (cast `/Game/Collab/Tech/Character/TopDownCharacter` (`GameplayStatics.GetPlayerCharacter` 0)))
    (set `self.PlayerRef` _astop_down_character)))

(fn `UpdateCharacter`
  (bind _skeletalmesh (`self.SkeletalMesh`))
  (bind _cupsm (`self.CupSM`))
  (switch `/Game/Collab/Tech/Character/E_Characters` (`self.Character`)
    (:`NewEnumerator0`
      (`SkinnedMeshComponent.SetSkinnedAssetAndUpdate` (`self.SkeletalMesh`) "/Game/Collab/Animation/Warrior/WarriorRig/Warrior_Rig_Unwrapped_v1.Warrior_Rig_Unwrapped_v1" true)
      (`PrimitiveComponent.SetMaterial` (`self.SkeletalMesh`) 0 "/Game/Collab/Animation/Warrior/WarriorRig/Materials/M_VesperFullsong.M_VesperFullsong")
      (`SkeletalMeshComponent.SetAnimation` _skeletalmesh "/Game/Collab/Animation/Tavern/Warrior_TavernIdle.Warrior_TavernIdle")
      (`SkeletalMeshComponent.SetAnimationMode` _skeletalmesh "AnimationSingleNode")
      (bind _returnvalue (`AddComponent|NODE_AddSkeletalMeshComponent-0`))
      (set `self.CupSM` _returnvalue)
      (`SkinnedMeshComponent.SetSkinnedAssetAndUpdate` _returnvalue "/Game/Collab/Animation/Tavern/Mug_TavernIdle.Mug_TavernIdle" true)
      (`SkeletalMeshComponent.SetAnimation` _returnvalue "/Game/Collab/Animation/Tavern/Mug_TavernIdle_Anim.Mug_TavernIdle_Anim")
      (`SceneComponent.K2_AttachToComponent` _returnvalue (`self.SkeletalMesh`) "TavernMugSocket" "SnapToTarget" "SnapToTarget" "SnapToTarget" true)
      (`self.K2_SetActorLocation` (`self.WarriorPosition`))
      (`self.K2_SetActorRotation` (`self.WarriorRotation`)))
    (:`NewEnumerator1`
      (`SkinnedMeshComponent.SetSkinnedAssetAndUpdate` (`self.SkeletalMesh`) "/Game/Collab/Animation/Paladin/Mesh/Paladin_Rig_Unwrapped_v1.Paladin_Rig_Unwrapped_v1" true)
      (`PrimitiveComponent.SetMaterial` (`self.SkeletalMesh`) 0 "/Game/Collab/Animation/Paladin/Textures/M_DarionFullsong.M_DarionFullsong")
      (`/Engine/EditorBlueprintResources/StandardMacros.IsValid` _cupsm
        (:`Is Valid`
          (`SceneComponent.SetVisibility` _cupsm false false))
        (:`Is Not Valid`
          _))
      (`SkeletalMeshComponent.SetAnimation` (`self.SkeletalMesh`) "/Game/Collab/Animation/Tavern/Paladin_Tavern_Idle.Paladin_Tavern_Idle")
      (`self.K2_SetActorLocation` (`self.PaladinPosition`))
      (`self.K2_SetActorRotation` (`self.PaladinRotation`)))))

(fn `UserConstructionScript`)