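; Base weapon Blueprint that resolves melee-range attacks for its owning player, whose reference is set through Init.
; Attack box-traces Pawn and WorldDynamic objects ahead of the weapon along player forward, gathering unique hit actors behind a re-entry guard.
; Enemy pawns take weapon damage plus player Strength, with both terms doubled and a message sent on crits.
; The non-enemy branch applies weapon damage alone, but has no damaged actor connected.
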(event `Init`
  (params (PlayerRef :type "/Game/Collab/Tech/Character/TopDownCharacter Object Reference"))
  (set `self.PlayerRef` PlayerRef))

(event `/Game/Collab/Tech/Weapon/BPI_WeaponActions.Attack`
  (params (Strength :type Integer) (`Crit?` :type Boolean))
  (bind _returnvalue (`self.K2_GetActorLocation` self))
  (set `self.CriticalHit` `Crit?`)
  (if (not (`self.CantAttack`))
    (set `self.CantAttack` true)
    (bind _outhits (`KismetSystemLibrary.BoxTraceMultiForObjects` _returnvalue (+ _returnvalue (* (`self.GetActorForwardVector` (`self.PlayerRef`)) 100.0)) (80.0 80.0 80.0) (struct) (`|MakeArray` "ObjectTypeQuery3" "ObjectTypeQuery2" :!type "EObjectTypeQuery Enum") false (`|MakeArray` (`self.PlayerRef`) :!type "Actor Object Reference") "None" true (struct :`R` 1.0 :`A` 1.0) (struct :`G` 1.0 :`A` 1.0) 0.5))
    (for _array_element _outhits
      (`KismetArrayLibrary.Array_AddUnique` (`self.TempHitActors`) (`.HitActor` (`GameplayStatics.BreakHitResult` _array_element))))
    (for _array_element_2 (`self.TempHitActors`)
      (if (`KismetMathLibrary.ClassIsChildOf` (`GameplayStatics.GetObjectClass` _array_element_2) "/Game/Collab/Tech/AI/Pawns/BaseEnemyPawn.BaseEnemyPawn_C")
        (if (`self.CriticalHit`)
          (`GameplayStatics.ApplyDamage` _array_element_2 (+ (* (`self.WeaponDamage`) 2.0) (* (`KismetMathLibrary.Conv_IntToDouble` (`.Strength_93_8F3DB7244A073A8BFCDF6AB4C9BB4C87` (break `/Game/Collab/Tech/Character/S_CharacterStats` (`/Game/Collab/Tech/Character/TopDownCharacter.CharacterStats` (`self.PlayerRef`))))) 2.0)) null (`self.PlayerRef`))
          (message `/Game/Collab/Tech/Interfaces/CombatInterface.BeenCrit` _array_element_2)
          (else
            (`GameplayStatics.ApplyDamage` _array_element_2 (+ (`self.WeaponDamage`) (`KismetMathLibrary.Conv_IntToDouble` (`.Strength_93_8F3DB7244A073A8BFCDF6AB4C9BB4C87` (break `/Game/Collab/Tech/Character/S_CharacterStats` (`/Game/Collab/Tech/Character/TopDownCharacter.CharacterStats` (`self.PlayerRef`)))))) null (`self.PlayerRef`))))
        (else
          ;[1 1 1] Just weapon damage
          (`GameplayStatics.ApplyDamage` null (`self.WeaponDamage`) null (`self.PlayerRef`)))))
    (set `self.CantAttack` false)
    (`KismetArrayLibrary.Array_Clear` (`self.TempHitActors`))))

(fn `UserConstructionScript`)