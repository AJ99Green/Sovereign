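; BP_DestructibleWall is a wall that highlights under the cursor and shatters when it takes any damage.
; Cursor hover on the Box toggles highlighting through BPAVisualSelection.
; AnyDamage applies a fixed heavy hit to the Destructible, pushing away from the damage causer regardless of damage amount, and disables its collision.
; If the Box is valid, it is destroyed after a short delay and the selection is cleared.
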(event `self.Box.OnBeginCursorOver`
  (params (TouchedComponent :type "PrimitiveComponent Object Reference"))
  (`/Game/Collab/Tech/SelectableObject/BPA_VisualSelection.Select` (`self.BPA_VisualSelection`) 6))

(event `self.Box.OnEndCursorOver`
  (params (TouchedComponent :type "PrimitiveComponent Object Reference"))
  (`/Game/Collab/Tech/SelectableObject/BPA_VisualSelection.Deselect` (`self.BPA_VisualSelection`)))

(event `self.ReceiveAnyDamage`
  (params (Damage :type "Float (single-precision)") (DamageType :type "DamageType Object Reference") (InstigatedBy :type "Controller Object Reference") (DamageCauser :type "Actor Object Reference"))
  (bind _returnvalue (`self.K2_GetActorLocation` DamageCauser))
  (bind _destructible (`self.Destructible`))
  (`DestructibleComponent.ApplyDamage` _destructible 5000.0 _returnvalue (* (`KismetMathLibrary.Normal` (- (`self.K2_GetActorLocation`) _returnvalue)) 5.0) 7000.0)
  (set `DestructibleComponent.LargeChunkThreshold` 120.0 _destructible)
  (`PrimitiveComponent.SetCollisionEnabled` _destructible "NoCollision")
  (`/Engine/EditorBlueprintResources/StandardMacros.IsValid` (`self.Box`)
    (:`Is Valid`
      (`KismetSystemLibrary.Delay` 2.0)
      (`ActorComponent.K2_DestroyComponent` (`self.Box`))
      (`/Game/Collab/Tech/SelectableObject/BPA_VisualSelection.Deselect` (`self.BPA_VisualSelection`)))))

(fn `UserConstructionScript`)