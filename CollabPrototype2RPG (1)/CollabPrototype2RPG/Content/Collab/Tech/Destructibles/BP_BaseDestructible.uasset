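; Base destructible prop that breaks apart when damaged or hit and can drop a randomized inventory item.
; Any damage turns on physics and applies radius damage to the destructible component from the player's location, while component hits apply a smaller directional impulse.
; Both paths call DropFromTable, gated once only on the hit path.
; DropFromTable optionally rolls an item and spawns BP_InventoryItem with rarity-based stats and level.
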(event `self.ReceiveBeginPlay`)

(event `self.ReceiveActorBeginOverlap`
  (params (OtherActor :type "Actor Object Reference")))

(event `self.ReceiveAnyDamage`
  (params (Damage :type "Float (single-precision)") (DamageType :type "DamageType Object Reference") (InstigatedBy :type "Controller Object Reference") (DamageCauser :type "Actor Object Reference"))
  (bind _dm_cube (`self.DM_Cube`))
  (`PrimitiveComponent.SetSimulatePhysics` _dm_cube true)
  (`DestructibleComponent.ApplyRadiusDamage` _dm_cube 2500.0 (`self.K2_GetActorLocation` (`GameplayStatics.GetPlayerPawn` 0)) 500.0 2500.0 true)
  (`self.DropFromTable`))

(event `self.DM_Cube.OnComponentHit`
  (params (HitComponent :type "PrimitiveComponent Object Reference") (OtherActor :type "Actor Object Reference") (OtherComp :type "PrimitiveComponent Object Reference") (NormalImpulse :type "Vector Structure") (Hit :type "HitResult Structure (by ref)"))
  (bind _returnvalue (`self.K2_GetActorLocation`))
  (`DestructibleComponent.ApplyDamage` (`self.DM_Cube`) 25.0 _returnvalue (- _returnvalue (`self.K2_GetActorLocation` (`GameplayStatics.GetPlayerPawn` 0))) 50.0)
  (`/Engine/EditorBlueprintResources/StandardMacros.DoOnce` false
    (:`Completed`
      (`self.DropFromTable`))))

(fn `DropFromTable`
  (bind (_returnvalue_location _returnvalue_rotation) (`KismetMathLibrary.BreakTransform` (`self.GetTransform`)))
  (if (`self.bShouldDropItems`)
    (bind (_out_item_data _out_item_id _bshoulddrop) (`/Game/Collab/Tech/Inventory/BP_InventoryLibrary.GenerateItemDrop`))
    (if _bshoulddrop
      (bind (_name _itemstatmodifiers _healamount _itemimage _description _itemtype _rarity) (break `/Game/Collab/Tech/Inventory/S_InventoryData` _out_item_data))
      (bind (_generatedvalues _out_itemlevel) (`/Game/Collab/Tech/Inventory/BP_InventoryLibrary.GenerateValuesFromBounds` _itemstatmodifiers _rarity -1 self))
      (`|SpawnActorFromClass` "/Game/Collab/Tech/Inventory/BP_InventoryItem.BP_InventoryItem_C" (`KismetMathLibrary.MakeTransform` _returnvalue_location _returnvalue_rotation) "AlwaysSpawn" "OverrideRootScale" null _out_item_id 0 _generatedvalues false _out_itemlevel null))))

(fn `UserConstructionScript`)