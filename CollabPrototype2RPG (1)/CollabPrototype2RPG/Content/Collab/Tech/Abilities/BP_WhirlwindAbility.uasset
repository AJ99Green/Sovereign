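; BP_WhirlwindAbility is an ability that deals area damage to enemies around the player character when used.
; UseAbility runs a multi sphere trace at player 0's location, with identical start and end, against WorldDynamic and Pawn objects.
; Hit actors derived from BaseEnemyPawn receive damage, with radius and amount both read from AbilityStats.
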(event `/Game/Collab/Tech/Abilities/BPI_Ability.UseAbility`
  (params (SpawnLocation :type "/Game/Collab/Tech/AI/Pawns/BaseEnemyPawn Object Reference"))
  (bind (_abilitystats_hitfx _abilitystats_cooldown _abilitystats_damage _abilitystats_damageradius) (break `/Game/Collab/Tech/Abilities/S_AbilityStats` (`self.AbilityStats`)))
  (bind _returnvalue (`self.K2_GetActorLocation` (`GameplayStatics.GetPlayerCharacter` 0)))
  ;[1 1 1] sphere cast & apply damage
  (bind _outhits (`KismetSystemLibrary.SphereTraceMultiForObjects` :`Start` _returnvalue :`End` _returnvalue :`Radius` _abilitystats_damageradius :`ObjectTypes` (`|MakeArray` "ObjectTypeQuery2" "ObjectTypeQuery3" :!type "EObjectTypeQuery Enum") :`DrawTime` 1.0))
  (for _array_element _outhits
    (if (`KismetMathLibrary.ClassIsChildOf` (`GameplayStatics.GetObjectClass` (`.HitActor` (`GameplayStatics.BreakHitResult` _array_element))) "/Game/Collab/Tech/AI/Pawns/BaseEnemyPawn.BaseEnemyPawn_C")
      (`GameplayStatics.ApplyDamage` (`.HitActor` (`GameplayStatics.BreakHitResult` _array_element)) _abilitystats_damage))))

(fn `UserConstructionScript`
  (`parent.UserConstructionScript`))