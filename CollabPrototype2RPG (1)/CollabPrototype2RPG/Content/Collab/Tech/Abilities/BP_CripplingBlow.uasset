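; BP_CripplingBlow is a player melee ability that damages and slows enemies in a short area in front of the character.
; UseAbility box-traces forward from player zero for pawns, dynamic objects and destructibles.
; Enemy pawns are gathered into a unique list, then each takes the ability's damage and a timed slow message.
; Non-enemy hits, meant for destructibles, take damage directly on every hit, and the list is cleared afterwards.
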(event `/Game/Collab/Tech/Abilities/BPI_Ability.UseAbility`
  (params (SpawnLocation :type "/Game/Collab/Tech/AI/Pawns/BaseEnemyPawn Object Reference"))
  (bind (_abilitystats_hitfx _abilitystats_cooldown _abilitystats_damage) (break `/Game/Collab/Tech/Abilities/Refactor/S_AbilityStats` (`self.AbilityStats`)))
  (bind _temphitactors (`self.TempHitActors`))
  (bind (_abilitystats_hitfx_2 _abilitystats_cooldown_2 _abilitystats_damage_2) (break `/Game/Collab/Tech/Abilities/Refactor/S_AbilityStats` (`self.AbilityStats`)))
  (bind _returnvalue (`self.K2_GetActorLocation` (`GameplayStatics.GetPlayerCharacter` 0)))
  (bind _outhits (`KismetSystemLibrary.BoxTraceMultiForObjects` _returnvalue (+ _returnvalue (* (`self.GetActorForwardVector` (`GameplayStatics.GetPlayerCharacter` 0)) 100.0)) (80.0 80.0 80.0) (struct) (`|MakeArray` "ObjectTypeQuery3" "ObjectTypeQuery2" "ObjectTypeQuery6" :!type "EObjectTypeQuery Enum") false (`|MakeArray` (`GameplayStatics.GetPlayerCharacter` 0) :!type "Actor Object Reference") "None" true (struct :`R` 1.0 :`A` 1.0) (struct :`G` 1.0 :`A` 1.0) 0.5))
  (for _array_element _outhits
    (if (`KismetMathLibrary.ClassIsChildOf` (`GameplayStatics.GetObjectClass` (`.HitActor` (`GameplayStatics.BreakHitResult` _array_element))) "/Game/Collab/Tech/AI/Pawns/BaseEnemyPawn.BaseEnemyPawn_C")
      (`KismetArrayLibrary.Array_AddUnique` (`self.TempHitActors`) (`.HitActor` (`GameplayStatics.BreakHitResult` _array_element)))
      (else
        ;[1 1 1] if the actor isn't an enemy, apply damage (for destructibles)
        (`GameplayStatics.ApplyDamage` (`.HitActor` (`GameplayStatics.BreakHitResult` _array_element)) _abilitystats_damage_2 null (`GameplayStatics.GetPlayerCharacter` 0)))))
  (for _array_element_2 _temphitactors
    (`GameplayStatics.ApplyDamage` _array_element_2 _abilitystats_damage null (`GameplayStatics.GetPlayerCharacter` 0))
    (message `/Game/Collab/Tech/Interfaces/CombatInterface.Slow Effect` _array_element_2 0.5 7.5))
  (`KismetArrayLibrary.Array_Clear` _temphitactors))

(fn `UserConstructionScript`
  (`parent.UserConstructionScript`))