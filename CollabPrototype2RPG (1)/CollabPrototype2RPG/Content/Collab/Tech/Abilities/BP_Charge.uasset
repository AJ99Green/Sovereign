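; Charge ability that teleports the player to the point under the cursor and damages actors around the landing.
; UseAbility samples ten points along the path, tracing down and projecting each onto the navmesh, and blocks the charge over unwalkable ground.
; After a short delay it moves the player, applies distance-falloff damage from AbilityStats and spawns HitFX, with debug drawing throughout.
; An enemy-targeted variant is disconnected, and ShowAbilityPath is empty.
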(event `/Game/Collab/Tech/Abilities/BPI_Ability.UseAbility`
  (params (SpawnLocation :type "/Game/Collab/Tech/AI/Pawns/BaseEnemyPawn Object Reference"))
  (bind _targetlocation (`self.TargetLocation`))
  (bind (_abilitystats_hitfx _abilitystats_cooldown _abilitystats_damage _abilitystats_damageradius) (break `/Game/Collab/Tech/Abilities/S_AbilityStats` (`self.AbilityStats`)))
  (bind _returnvalue (`self.K2_GetActorLocation` (`GameplayStatics.GetPlayerCharacter` 0)))
  (bind _output_get (set `self.TargetLocation` (`.Location` (`GameplayStatics.BreakHitResult` (`PlayerController.GetHitResultUnderCursorByChannel` (`GameplayStatics.GetPlayerController` 0) "TraceTypeQuery1" true)))))
  (`KismetSystemLibrary.DrawDebugLine` _returnvalue _output_get (struct :`R` 1.0 :`B` 0.0409 :`A` 1.0) 10.0 1.0)
  (for _index (range 10)
    (bind _returnvalue_2 (+ (* (`KismetMathLibrary.GetDirectionUnitVector` _returnvalue (`self.TargetLocation`)) (* _index (/ (`KismetMathLibrary.Vector_Distance` _returnvalue (`self.TargetLocation`)) 10.0))) _returnvalue))
    (bind _outhit (`KismetSystemLibrary.LineTraceSingle` :`Start` _returnvalue_2 :`End` (- _returnvalue_2 (0.0 0.0 5000.0)) :`TraceChannel` "TraceTypeQuery1" :`DrawDebugType` "ForDuration" :`TraceColor` (struct :`R` 1.0 :`G` 0.046773 :`A` 1.0) :`TraceHitColor` (struct :`R` 1.0 :`G` 0.097409 :`A` 1.0)))
    (bind _outactors (`GameplayStatics.GetAllActorsOfClass` "/Script/NavigationSystem.RecastNavMesh"))
    (if (`KismetArrayLibrary.Array_IsValidIndex` _outactors)
      (if (not (`.ReturnValue` (`NavigationSystemV1.K2_ProjectPointToNavigation` (`.Location` (`GameplayStatics.BreakHitResult` _outhit)) (`|GetArrayItem` _outactors) null (20.0 20.0 200.0))))
        (`KismetSystemLibrary.PrintString` "---Charge is blocked by unwalkable terrain")
        (set `self.bCanCharge` false)
        (break))))
  (if (`self.bCanCharge`)
    (`KismetSystemLibrary.PrintString` "---Player charges forward---")
    (`KismetSystemLibrary.Delay` 0.5)
    ;[1 1 1] this is really weird atm
    (`self.K2_SetActorLocation` (`GameplayStatics.GetPlayerCharacter` 0) (+ _targetlocation (0.0 0.0 10.0)) true true)
    (bind _outactors_2 (`KismetSystemLibrary.SphereOverlapActors` _targetlocation 500.0 (`|MakeArray` "ObjectTypeQuery3" "ObjectTypeQuery6" "ObjectTypeQuery2" "ObjectTypeQuery1" :!type "EObjectTypeQuery Enum") null (`|MakeArray` (`GameplayStatics.GetPlayerCharacter` 0) :!type "Actor Object Reference")))
    (`KismetSystemLibrary.DrawDebugSphere` (`self.TargetLocation`) 500.0 12 (struct :`R` 1.0 :`G` 1.0 :`B` 1.0 :`A` 1.0) 2.0 1.0)
    (for _array_element _outactors_2
      (`KismetSystemLibrary.Delay` 0.2)
      (bind _returnvalue_3 (`KismetMathLibrary.Vector_Distance` (`self.K2_GetActorLocation` _array_element) (`self.TargetLocation`)))
      (bind _returnvalue_4 (`GameplayStatics.ApplyDamage` _array_element (select `bool` (> _returnvalue_3 _abilitystats_damageradius) :`false` (* (`KismetMathLibrary.Abs` (- 1.0 (/ _returnvalue_3 _abilitystats_damageradius))) _abilitystats_damage)) null (`GameplayStatics.GetPlayerPawn` 0)))
      (`KismetSystemLibrary.PrintString` (`KismetStringLibrary.Conv_DoubleToString` _returnvalue_4)))
    (`GameplayStatics.SpawnEmitterAtLocation` _abilitystats_hitfx (- (`self.TargetLocation`) (0.0 0.0 106.25)))))

(event `/Game/Collab/Tech/Abilities/BPI_Ability.ShowAbilityPath`)

(fn `UserConstructionScript`
  (`parent.UserConstructionScript`))