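; BP_Fleshrender is an ability that damages actors in a cone from the player toward the cursor.
; UseAbility approximates the cone with chained multi-sphere traces over a fixed range, widening linearly from start to end radius, with debug drawing.
; Hits from the loop's traces take AbilityStats damage once via ActorsAlreadyHit; the first trace's hits are ignored.
; A separate ApplyDamage helper exists but UseAbility applies damage inline.
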(event `/Game/Collab/Tech/Abilities/BPI_Ability.UseAbility`
  (params (SpawnLocation :type "/Game/Collab/Tech/AI/Pawns/BaseEnemyPawn Object Reference"))
  (bind (_abilitystats_hitfx _abilitystats_cooldown _abilitystats_damage) (break `/Game/Collab/Tech/Abilities/Refactor/S_AbilityStats` (`self.AbilityStats`)))
  (bind _conetraceoffset (`self.ConeTraceOffset`))
  (bind _returnvalue (`self.K2_GetActorLocation` (`GameplayStatics.GetPlayerCharacter` 0)))
  (bind _returnvalue_2 (/ 1.0 (`KismetMathLibrary.Conv_IntToDouble` (`self.ConeSteps`))))
  (bind _returnvalue_3 (`KismetMathLibrary.GetDirectionUnitVector` _returnvalue (`.Location` (`GameplayStatics.BreakHitResult` (`PlayerController.GetHitResultUnderCursorByChannel` (`GameplayStatics.GetPlayerController` 0) "TraceTypeQuery1" true)))))
  (bind _returnvalue_4 (+ (* _returnvalue_3 (* 500.0 _returnvalue_2)) _conetraceoffset))
  (bind _returnvalue_5 (+ (* _returnvalue_3 (* 500.0 (/ 1.0 (`KismetMathLibrary.Conv_IntToDouble` (`self.ConeSteps`))))) _returnvalue))
  ;[1 1 1] Via https://forums.unrealengine.com/community/community-content-tools-and-tutorials/113115-cone-trace-with-proper-distance-steps-and-start-end-radius-size-controls
  (`KismetSystemLibrary.SphereTraceMulti` (`self.K2_GetActorLocation` (`GameplayStatics.GetPlayerCharacter` 0)) _returnvalue_5 (`self.StartRadius`) "TraceTypeQuery1" false (`|MakeArray` self :!type "Actor Object Reference") "ForDuration" true (struct :`G` 0.094117 :`B` 1.0 :`A` 1.0))
  (set `self.ConeTraceOffset` _returnvalue_5)
  ;;[1 1 1] Start at second iteration of spheres as first is already traced before
  (for _index (range 2 (+ (`self.ConeSteps`) 1))
    (bind _outhits (`KismetSystemLibrary.SphereTraceMulti` _conetraceoffset _returnvalue_4 (`KismetMathLibrary.MapRangeClamped` (* _index _returnvalue_2) 0.0 1.0 (`self.StartRadius`) (`self.EndRadius`)) "TraceTypeQuery1" false (`|MakeArray` self :!type "Actor Object Reference") "ForDuration"))
    ;;[1 1 1] set new offset to previous sphere trace point
    (set `self.ConeTraceOffset` _returnvalue_4)
    (for _array_element _outhits
      (bind (_bblockinghit _binitialoverlap _time _distance _location _impactpoint _normal _impactnormal _physmat _hitactor) (`GameplayStatics.BreakHitResult` _array_element))
      (if (not (`KismetArrayLibrary.Array_Contains` (`self.ActorsAlreadyHit`) _hitactor))
        (`KismetArrayLibrary.Array_Add` (`self.ActorsAlreadyHit`) _hitactor)
        (`GameplayStatics.ApplyDamage` _hitactor _abilitystats_damage null (`GameplayStatics.GetPlayerCharacter` 0))))))

(fn `ApplyDamage`
  (params (HitActors :type "Array of HitResult Structure"))
  (locals (Local_HitActors :type "Array of Actor Object Reference"))
  (bind (_abilitystats_hitfx _abilitystats_cooldown _abilitystats_damage) (break `/Game/Collab/Tech/Abilities/Refactor/S_AbilityStats` (`self.AbilityStats`)))
  (for _array_element HitActors
    (bind (_bblockinghit _binitialoverlap _time _distance _location _impactpoint _normal _impactnormal _physmat _hitactor) (`GameplayStatics.BreakHitResult` _array_element))
    (if (not (`KismetArrayLibrary.Array_Contains` (`local.Local_HitActors`) _hitactor))
      (`GameplayStatics.ApplyDamage` _hitactor _abilitystats_damage null (`GameplayStatics.GetPlayerCharacter` 0))
      (`KismetArrayLibrary.Array_Add` (`local.Local_HitActors`) _hitactor)))
  (return))

(fn `UserConstructionScript`
  (`parent.UserConstructionScript`))