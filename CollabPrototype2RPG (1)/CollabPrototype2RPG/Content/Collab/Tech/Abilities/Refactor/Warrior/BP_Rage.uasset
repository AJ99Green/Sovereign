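; Warrior Rage ability that, when used at full rage, plays a montage and attached effect and doubles Strength, both Defences and Attack Speed.
; RageIncrease builds the clamped meter; use below max resets the ability after a brief delay.
; While raging, a one-second timer drains the meter at an escalating rate.
; At zero, StopRage clears the effect, restores the pre-rage stat snapshot and signals ability finished for cooldown.
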(event `/Game/Collab/Tech/Abilities/Refactor/BPI_AbilityInteraction.Use`
  (params (PlayerRef :type "/Game/Collab/Tech/Character/TopDownCharacter Object Reference"))
  (bind ((`CurrentRage_51_74B754C34EC58FBC8FD86594D1FDE480` _currentrage) (`MaxRage_52_88B400B14BA7A68EA73ECCB7930A4A25` _maxrage)) (break `/Game/Collab/Tech/Abilities/Refactor/S_AbilityStats` (`self.AbilityStats`)))
  (set `self.PlayerRef` PlayerRef)
  (if (>= _currentrage _maxrage)
    (`self.Rage`)
    (else
      (`KismetSystemLibrary.Delay` 0.1)
      (`/Game/Collab/Tech/Abilities/Refactor/BPA_AbilityManager.ResetAbility` (`/Game/Collab/Tech/Character/TopDownCharacter.BPA_AbilityManager` (`self.PlayerRef`)) (`GameplayStatics.GetObjectClass` self)))))

(event `/Game/Collab/Tech/Abilities/Refactor/BPI_AbilityInteraction.RageIncrease`
  (params (IncreaseAmount :type "Float (single-precision)"))
  (`self.ModifyRage` IncreaseAmount true))

(fn `ModifyRage`
  (params (ChangeAmount :type "Float (double-precision)") (`Positive?` :type Boolean))
  (locals (TempRage :type "Float (double-precision)"))
  (bind ((`CurrentRage_51_74B754C34EC58FBC8FD86594D1FDE480` _currentrage) (`MaxRage_52_88B400B14BA7A68EA73ECCB7930A4A25` _maxrage)) (break `/Game/Collab/Tech/Abilities/Refactor/S_AbilityStats` (`self.AbilityStats`)))
  (bind ((`CurrentRage_51_74B754C34EC58FBC8FD86594D1FDE480` _currentrage_2) (`MaxRage_52_88B400B14BA7A68EA73ECCB7930A4A25` _maxrage_2)) (break `/Game/Collab/Tech/Abilities/Refactor/S_AbilityStats` (`self.AbilityStats`)))
  (if `Positive?`
    (set `local.TempRage` (`KismetMathLibrary.FClamp` (+ _currentrage_2 ChangeAmount) 0.0 _maxrage_2))
    (else
      (set `local.TempRage` (`KismetMathLibrary.FClamp` (- _currentrage ChangeAmount) 0.0 _maxrage))))
  (setmembers `/Game/Collab/Tech/Abilities/Refactor/S_AbilityStats` :`StructRef` (`self.AbilityStats`) :`CurrentRage` (`local.TempRage`))
  (`self.RageModified` ChangeAmount `Positive?`))

(fn `Rage`
  (bind _playerref (`self.PlayerRef`))
  (bind _playerref_2 (`self.PlayerRef`))
  (bind ((`Strength_93_8F3DB7244A073A8BFCDF6AB4C9BB4C87` _strength) (`PhysicalDefence_90_BE7A84504913CF82FAA82D9772ABFED8` _physicaldefence) (`MagicalDefence_91_E333A3284F2669A09B8A5FA2B7207107` _magicaldefence) (`AttackSpeed_85_A5B150B04D39E430AB909CA9E5D32B89` _attackspeed)) (break `/Game/Collab/Tech/Character/S_CharacterStats` (`/Game/Collab/Tech/Character/TopDownCharacter.CharacterStats` (`self.PlayerRef`))))
  ;[1 1 1] Play animation
  (`Character.PlayAnimMontage` (`self.PlayerRef`) (`self.GetAnimation`) 1.0 "None")
  ;[1 1 1] Spawn Effect
  (bind _returnvalue (`GameplayStatics.SpawnEmitterAttached` (`.HitFX_3_A4D89F414F998065D4C18EB26A3183FF` (break `/Game/Collab/Tech/Abilities/Refactor/S_AbilityStats` (`self.AbilityStats`))) (`Character.Mesh` (`self.PlayerRef`)) "None" (0.0 0.0 50.0) (struct) (2.0 2.0 2.0)))
  (set `self.RageEffect` _returnvalue)
  ;[1 1 1] Update Rage State
  (setmembers `/Game/Collab/Tech/Abilities/Refactor/S_AbilityStats` :`StructRef` (`self.AbilityStats`) :`Raging` true)
  (`self.RageStateChanged` true)
  ;[1 1 1] Buff Stats
  (set `/Game/Collab/Tech/Character/TopDownCharacter.CurrentStats` (`/Game/Collab/Tech/Character/TopDownCharacter.CharacterStats` _playerref) _playerref)
  (`/Game/Collab/Tech/Character/TopDownCharacter.ModifyStrength` _playerref_2 _strength true)
  (`/Game/Collab/Tech/Character/TopDownCharacter.ModifyDefence` _playerref_2 _physicaldefence true _magicaldefence true)
  (`/Game/Collab/Tech/Character/TopDownCharacter.ModifyAttackSpeed` _playerref_2 _attackspeed true)
  ;[1 1 1] Start Rage Reduce Timer
  (bind _returnvalue_2 (`KismetSystemLibrary.K2_SetTimerDelegate` (`|CreateDelegate` :!event `ReduceRage`) 1.0 true))
  (set `self.ReduceTimerHandle` _returnvalue_2))

(fn `ReduceRage`
  (`self.ModifyRage` (`self.RageReducePerSec`))
  (if (<= (`.CurrentRage_51_74B754C34EC58FBC8FD86594D1FDE480` (break `/Game/Collab/Tech/Abilities/Refactor/S_AbilityStats` (`self.AbilityStats`))) 0.0)
    (`self.StopRage`)
    (else
      (set `self.RageReducePerSec` (+ (`self.RageReducePerSec`) 5.0)))))

(fn `ResetStats`
  (bind _playerref (`self.PlayerRef`))
  (set `/Game/Collab/Tech/Character/TopDownCharacter.CharacterStats` (`/Game/Collab/Tech/Character/TopDownCharacter.CurrentStats` _playerref) _playerref)
  (`/Game/Collab/Tech/Character/TopDownCharacter.HealthModified` (`self.PlayerRef`) 0.0 false)
  (`/Game/Collab/Tech/Character/TopDownCharacter.DefenceModified` (`self.PlayerRef`) 0.0 false 0.0 false)
  (`/Game/Collab/Tech/Character/TopDownCharacter.AttackSpeedModified` (`self.PlayerRef`) 0.0 false))

(fn `StopRage`
  ;[1 1 1] Stop Timer
  (`KismetSystemLibrary.K2_ClearAndInvalidateTimerHandle` (`self.ReduceTimerHandle`))
  ;[1 1 1] Destroy Effect
  (`ActorComponent.K2_DestroyComponent` (`self.RageEffect`))
  ;[1 1 1] Update Rage State
  (setmembers `/Game/Collab/Tech/Abilities/Refactor/S_AbilityStats` :`StructRef` (`self.AbilityStats`) :`Raging` false)
  (`self.RageStateChanged` false)
  ;[1 1 1] Reset Current Rage
  (`self.ModifyRage` (`.CurrentRage_51_74B754C34EC58FBC8FD86594D1FDE480` (break `/Game/Collab/Tech/Abilities/Refactor/S_AbilityStats` (`self.AbilityStats`))))
  ;[1 1 1] Set Stats Back to Normal
  (`self.ResetStats`)
  ;[1 1 1] Rage Finished begin cooldown
  (`self.OnAbilityFinished` self))

(fn `UserConstructionScript`
  (`parent.UserConstructionScript`))