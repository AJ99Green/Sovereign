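; Warrior Fleshrender ability: a frontal melee strike that damages one target and makes enemies bleed.
; Use plays the montage, waits until shortly before it ends, then spawns a hit effect at ground level and box-traces ahead, with debug drawing on.
; Enemies take crit-checked damage and receive crit and bleed messages; any other hit takes base damage.
; Both branches signal ability completion, with tuning read from AbilityStats.
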(event `/Game/Collab/Tech/Abilities/Refactor/BPI_AbilityInteraction.Use`
  (params (PlayerRef :type "/Game/Collab/Tech/Character/TopDownCharacter Object Reference"))
  (bind _playerref (`self.PlayerRef`))
  (bind _playerref_2 (`self.PlayerRef`))
  (bind ((`BleedDamage_57_336050D447FDF3E5CF518EB17546B0AD` _bleeddamage) (`BleedTime_58_322760B14A17E033E410798D09F48FC2` _bleedtime)) (break `/Game/Collab/Tech/Abilities/Refactor/S_AbilityStats` (`self.AbilityStats`)))
  (bind ((`Radius_60_961B55264A85427CF39F2E901AD90497` _radius)) (break `/Game/Collab/Tech/Abilities/Refactor/S_AbilityStats` (`self.AbilityStats`)))
  (bind (_returnvalue_roll _returnvalue_pitch _returnvalue_yaw) (`KismetMathLibrary.BreakRotator` (`self.K2_GetActorRotation` (`self.PlayerRef`))))
  (bind _returnvalue (`self.K2_GetActorLocation` _playerref))
  (bind (_returnvalue_x _returnvalue_y _returnvalue_z) (`KismetMathLibrary.BreakVector` (`self.K2_GetActorLocation` _playerref_2)))
  ;[1 1 1] On flesh render used
  (bind _output_get (set `self.PlayerRef` PlayerRef))
  ;;[1 1 1] Play anim montage and delay for part of the animation so damage is dealt at correct point
  (bind _returnvalue_2 (`Character.PlayAnimMontage` _output_get (`.Animation_38_B819E5424B8DBA9AD91893A57EC41E4A` (break `/Game/Collab/Tech/Abilities/Refactor/S_AbilityStats` (`self.AbilityStats`))) 1.0 "None"))
  (`KismetSystemLibrary.Delay` (- _returnvalue_2 0.3))
  ;;[1 1 1] Spawn Effect
  (`GameplayStatics.SpawnEmitterAtLocation` (`.HitFX_3_A4D89F414F998065D4C18EB26A3183FF` (break `/Game/Collab/Tech/Abilities/Refactor/S_AbilityStats` (`self.AbilityStats`))) (+ (`KismetMathLibrary.MakeVector` _returnvalue_x _returnvalue_y (- _returnvalue_z (.z (`.BoxExtent` (`self.GetActorBounds` _playerref_2 true false))))) (* (`self.GetActorForwardVector` _playerref_2) 100.0)) (`KismetMathLibrary.MakeRotator` _returnvalue_roll _returnvalue_pitch (+ _returnvalue_yaw 120.0)) (0.5 0.5 0.5))
  ;;[1 1 1] Box trace for object in front of player
  (bind _outhit (`KismetSystemLibrary.BoxTraceSingleForObjects` _returnvalue (+ _returnvalue (* (`self.GetActorForwardVector` _playerref) 100.0)) (`KismetMathLibrary.MakeVector` _radius _radius _radius) (struct) (`|MakeArray` "ObjectTypeQuery3" "ObjectTypeQuery2" "ObjectTypeQuery6" :!type "EObjectTypeQuery Enum") false (`|MakeArray` (`self.PlayerRef`) :!type "Actor Object Reference") "Persistent" true (struct :`R` 1.0 :`A` 1.0) (struct :`G` 1.0 :`A` 1.0) 0.5))
  ;;[1 1 1] For object hit set variable, and see if type of enemy
  (set `self.ObjectHit` (`.HitActor` (`GameplayStatics.BreakHitResult` _outhit)))
  (if (`KismetMathLibrary.ClassIsChildOf` (`GameplayStatics.GetObjectClass` (`self.ObjectHit`)) "/Game/Collab/Tech/AI/Pawns/BaseEnemyPawn.BaseEnemyPawn_C")
    (bind _iscrit_ (`self.IsCrit?` (`self.ObjectHit`)))
    (if _iscrit_
      (message `/Game/Collab/Tech/Interfaces/CombatInterface.BeenCrit` (`self.ObjectHit`)))
    (bind _damage (`self.CalculateDamage` _iscrit_))
    (`GameplayStatics.ApplyDamage` (`self.ObjectHit`) _damage null (`self.PlayerRef`))
    (message `/Game/Collab/Tech/Interfaces/CombatInterface.Bleed Effect` (`self.ObjectHit`) _bleeddamage _bleedtime)
    (`self.OnAbilityFinished` self)
    (else
      ;;[1 1 1] if the actor isn't an enemy, apply damage (for destructibles)
      (`GameplayStatics.ApplyDamage` (`self.ObjectHit`) (`.Damage_9_F3F577364B193D803DFA64A17579BBCC` (break `/Game/Collab/Tech/Abilities/Refactor/S_AbilityStats` (`self.AbilityStats`))) null (`self.PlayerRef`))
      (`self.OnAbilityFinished` self))))

(fn `UserConstructionScript`
  (`parent.UserConstructionScript`))