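; Warrior Stampede ability that charges the player to the aimed location, damaging whatever is in the path.
; When aiming finishes, a timeline lerps the player from start to target, raised by the pawn's bounds, without sweeping.
; Each update runs a sphere overlap, hitting each actor only once: enemies take knockback and crit-aware damage, other actors take base damage.
; The ability signals completion when the timeline ends.
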(event `OnMoveTo`
  (params (StartingLocation :type "Vector Structure") (TargetLocation :type "Vector Structure"))
  (bind _objecthit (`self.ObjectHit`))
  ;[1 1 1] On Move To called when aiming has finished
  (`KismetArrayLibrary.Array_Clear` (`self.HitActors`))
  (`TimelineComponent.SetPlayRate` (`self.MoveTimeline`) 2.0)
  (bind (_direction _floatlerp) (`Timeline|MoveTimeline` :!via `PlayFromStart`)
    (:`Update`
      (bind _returnvalue (`KismetMathLibrary.VLerp` StartingLocation TargetLocation _floatlerp))
      (`self.K2_SetActorLocation` (`self.PlayerRef`) _returnvalue false false)
      (bind _outactors (`KismetSystemLibrary.SphereOverlapActors` _returnvalue 150.0 (`|MakeArray` "ObjectTypeQuery2" "ObjectTypeQuery3" "ObjectTypeQuery6" :!type "EObjectTypeQuery Enum") null (`|MakeArray` (`self.PlayerRef`) :!type "Actor Object Reference")))
      ;;[1 1 1] Only deal damage to each hit actor once
      (for _array_element _outactors
        (set `self.ObjectHit` _array_element)
        (if (not (`KismetArrayLibrary.Array_Contains` (`self.HitActors`) (`self.ObjectHit`)))
          (`KismetArrayLibrary.Array_Add` (`self.HitActors`) _objecthit)
          (if (`KismetMathLibrary.ClassIsChildOf` (`GameplayStatics.GetObjectClass` _objecthit) "/Game/Collab/Tech/AI/Pawns/BaseEnemyPawn.BaseEnemyPawn_C")
            (message `/Game/Collab/Tech/Interfaces/CombatInterface.Knockback` (`self.ObjectHit`) (`self.GetActorForwardVector` (`self.PlayerRef`)))
            (bind _iscrit_ (`self.IsCrit?` (`self.ObjectHit`)))
            (if _iscrit_
              (message `/Game/Collab/Tech/Interfaces/CombatInterface.BeenCrit` (`self.ObjectHit`)))
            (bind _damage (`self.CalculateDamage` _iscrit_))
            (`GameplayStatics.ApplyDamage` (`self.ObjectHit`) _damage null (`self.PlayerRef`))
            (else
              ;;;[1 1 1] if the actor isn't an enemy, apply damage (for destructibles)
              (`GameplayStatics.ApplyDamage` (`self.ObjectHit`) (`.Damage_9_F3F577364B193D803DFA64A17579BBCC` (break `/Game/Collab/Tech/Abilities/Refactor/S_AbilityStats` (`self.AbilityStats`))) null (`self.PlayerRef`)))))))
    (:`Finished`
      ;;[1 1 1] At the end of charge when player has finished charging
      (`self.OnAbilityFinished` self))))

(fn `OnAimFinished`
  (params (AimPosition :type "Vector Structure"))
  (bind _returnvalue (`GameplayStatics.GetPlayerPawn` 0))
  (bind (_returnvalue_x _returnvalue_y _returnvalue_z) (`KismetMathLibrary.BreakVector` (`SceneComponent.K2_GetComponentLocation` (`self.AimingNS`))))
  (`self.OnMoveTo` (`self.K2_GetActorLocation` _returnvalue) (`KismetMathLibrary.MakeVector` _returnvalue_x _returnvalue_y (+ _returnvalue_z (.z (`.BoxExtent` (`self.GetActorBounds` _returnvalue true false)))))))

(fn `UserConstructionScript`
  (`parent.UserConstructionScript`))