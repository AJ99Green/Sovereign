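; Warrior whirlwind ability that damages all enemies around the player for the length of the spin.
; On use it plays the montage, attaches a scaled particle effect and starts a looping timer, then clears both and signals ability finished after the stat-driven duration.
; Each tick sphere-traces around the player, filters for BaseEnemyPawn children, rolls crits with a crit message, and applies calculated damage.
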(event `/Game/Collab/Tech/Abilities/Refactor/BPI_AbilityInteraction.Use`
  (params (PlayerRef :type "/Game/Collab/Tech/Character/TopDownCharacter Object Reference"))
  ;[1 1 1] On whirlwind used
  (bind _output_get (set `self.PlayerRef` PlayerRef))
  ;;[1 1 1] Play whirlwind animation montage
  (`Character.PlayAnimMontage` _output_get (`.Animation_60_FA2EA33D48A6E6C942BF209C78FFCB00` (break `/Game/Collab/Tech/Abilities/Refactor/S_AbilityStats` (`self.AbilityStats`))) 1.0 "None")
  ;;[1 1 1] Spawn whirlwind effect
  (bind _returnvalue (`GameplayStatics.SpawnEmitterAttached` (`.HitFX_3_A4D89F414F998065D4C18EB26A3183FF` (break `/Game/Collab/Tech/Abilities/Refactor/S_AbilityStats` (`self.AbilityStats`))) (`Actor.RootComponent` (`self.PlayerRef`)) "None" (0.0 0.0 0.0) (struct) (2.0 2.0 2.0) "SnapToTarget"))
  (set `self.SpawnedEffect` _returnvalue)
  ;;[1 1 1] Apply repeating damage of whirlwind spin
  (bind _returnvalue_2 (`KismetSystemLibrary.K2_SetTimerDelegate` (`|CreateDelegate` :!event `ApplyDamageInRadius`) 0.2 true))
  ;;[1 1 1] Wait for how long the ability lasts
  (`KismetSystemLibrary.Delay` (`.AbilityDuration_19_E06109C245A749342E1A3BBC0C674573` (break `/Game/Collab/Tech/Abilities/Refactor/S_AbilityStats` (`self.AbilityStats`))))
  (`KismetSystemLibrary.K2_ClearAndInvalidateTimerHandle` _returnvalue_2)
  (`ActorComponent.K2_DestroyComponent` (`self.SpawnedEffect`))
  (`self.OnAbilityFinished` self))

(event `ApplyDamageInRadius`
  (bind _returnvalue (`self.K2_GetActorLocation` (`self.PlayerRef`)))
  ;[1 1 1] Apply damage in ability radius
  ;;[1 1 1] Multi sphere trace for objects in whirlwind range
  (bind _outhits (`KismetSystemLibrary.SphereTraceMultiForObjects` :`Start` _returnvalue :`End` _returnvalue :`Radius` (`.DamageRadius_11_961B55264A85427CF39F2E901AD90497` (break `/Game/Collab/Tech/Abilities/Refactor/S_AbilityStats` (`self.AbilityStats`))) :`ObjectTypes` (`|MakeArray` "ObjectTypeQuery2" "ObjectTypeQuery3" :!type "EObjectTypeQuery Enum") :`DrawTime` 1.0))
  ;;[1 1 1] For each object in range check to see if type of enemy
  (for _array_element _outhits
    (if (`KismetMathLibrary.ClassIsChildOf` (`GameplayStatics.GetObjectClass` (`.HitActor` (`GameplayStatics.BreakHitResult` _array_element))) "/Game/Collab/Tech/AI/Pawns/BaseEnemyPawn.BaseEnemyPawn_C")
      ;;[1 1 1] Check to see if crit?
      (bind _iscrit_ (`self.IsCrit?` (`.HitActor` (`GameplayStatics.BreakHitResult` _array_element))))
      (if _iscrit_
        (message `/Game/Collab/Tech/Interfaces/CombatInterface.BeenCrit` (`.HitActor` (`GameplayStatics.BreakHitResult` _array_element))))
      ;;[1 1 1] Calculate and apply damage
      (bind _damage (`self.CalculateDamage` _iscrit_))
      (`GameplayStatics.ApplyDamage` (`.HitActor` (`GameplayStatics.BreakHitResult` _array_element)) _damage null (`self.PlayerRef`)))))

(fn `UserConstructionScript`
  (`parent.UserConstructionScript`))