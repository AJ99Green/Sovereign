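; BP_OldDash is a warrior dash ability that instantly teleports the player character toward the mouse cursor.
; On Use, it calls the parent, then finds a point a fixed distance along the direction to the cursor's visibility-trace hit and draws a debug line to it.
; That point is projected onto the navmesh with a wide extent, and the character moves there without sweeping only if projection succeeds.
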(event `/Game/Collab/Tech/Abilities/Refactor/BPI_AbilityInteraction.Use`
  (params (PlayerRef :type "/Game/Collab/Tech/Character/TopDownCharacter Object Reference"))
  (bind _returnvalue (`self.K2_GetActorLocation` (`GameplayStatics.GetPlayerCharacter` 0)))
  (bind _returnvalue_2 (+ (* (`KismetMathLibrary.GetDirectionUnitVector` _returnvalue (`.Location` (`GameplayStatics.BreakHitResult` (`PlayerController.GetHitResultUnderCursorByChannel` (`GameplayStatics.GetPlayerController` 0) "TraceTypeQuery1" true)))) 500.0) _returnvalue))
  (bind (_projectedlocation _returnvalue_3) (`NavigationSystemV1.K2_ProjectPointToNavigation` _returnvalue_2 null null (1000.0 1000.0 1000.0)))
  (`parent.Use` null)
  (`KismetSystemLibrary.DrawDebugLine` _returnvalue _returnvalue_2 (struct :`R` 1.0 :`B` 0.04282 :`A` 1.0) 1.0)
  ;[1 1 1] if on navmesh dont do rest
  (if _returnvalue_3
    (`self.K2_SetActorLocation` (`GameplayStatics.GetPlayerCharacter` 0) _projectedlocation false true)))

(fn `UserConstructionScript`
  (`parent.UserConstructionScript`))