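; Warrior Earthshaker ability that damages enemies in a cone toward the cursor.
; On use it turns the player to the cached cursor point, plays the cast montage and waits until shortly before it ends.
; Chained sphere traces with growing radii approximate the cone, damaging each enemy once with possible crits; the first trace's hits go unused.
; It then signals that the ability has finished.
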(event `/Game/Collab/Tech/Abilities/Refactor/BPI_AbilityInteraction.Use`
  (params (PlayerRef :type "/Game/Collab/Tech/Character/TopDownCharacter Object Reference"))
  (bind (_returnvalue_roll _returnvalue_pitch) (`KismetMathLibrary.BreakRotator` (`self.K2_GetActorRotation` (`self.PlayerRef`))))
  (bind _returnvalue (`self.K2_GetActorLocation` (`self.PlayerRef`)))
  (bind (_returnvalue_roll_2 _returnvalue_pitch_2 _returnvalue_yaw) (`KismetMathLibrary.BreakRotator` (`KismetMathLibrary.FindLookAtRotation` (`self.K2_GetActorLocation` (`self.PlayerRef`)) (`self.CachedCursorPos`))))
  (bind _returnvalue_2 (`KismetMathLibrary.GetDirectionUnitVector` _returnvalue (`self.CachedCursorPos`)))
  (bind _returnvalue_3 (+ (* _returnvalue_2 (* 500.0 (/ 1.0 (`KismetMathLibrary.Conv_IntToDouble` (`self.ConeSteps`))))) (`self.ConeTraceOffset`)))
  (bind _returnvalue_4 (+ (* _returnvalue_2 (* 500.0 (/ 1.0 (`KismetMathLibrary.Conv_IntToDouble` (`self.ConeSteps`))))) _returnvalue))
  ;[1 1 1] On Earthshaker used, cache hit cursor result for direction of cone trace
  (set `self.PlayerRef` PlayerRef)
  (`KismetArrayLibrary.Array_Clear` (`self.ActorsAlreadyHit`))
  (set `self.CachedCursorPos` (`.Location` (`GameplayStatics.BreakHitResult` (`PlayerController.GetHitResultUnderCursorByChannel` (`GameplayStatics.GetPlayerController` 0) "TraceTypeQuery1" true))))
  ;[1 1 1] set actor rotation to the direction we're using the ability in
  (`self.K2_SetActorRotation` (`self.PlayerRef`) (`KismetMathLibrary.MakeRotator` _returnvalue_roll _returnvalue_pitch _returnvalue_yaw) false)
  ;[1 1 1] play cast montage
  (bind _returnvalue_5 (`Character.PlayAnimMontage` (`self.PlayerRef`) (`.Animation_38_B819E5424B8DBA9AD91893A57EC41E4A` (break `/Game/Collab/Tech/Abilities/Refactor/S_AbilityStats` (`self.AbilityStats`))) 1.0 "None"))
  (`KismetSystemLibrary.Delay` (- _returnvalue_5 0.3))
  ;[1 1 1] initial sphere trace
  (`KismetSystemLibrary.SphereTraceMulti` (`self.K2_GetActorLocation` (`self.PlayerRef`)) _returnvalue_4 (`.Radius_60_961B55264A85427CF39F2E901AD90497` (break `/Game/Collab/Tech/Abilities/Refactor/S_AbilityStats` (`self.AbilityStats`))) "TraceTypeQuery1" false (`|MakeArray` self :!type "Actor Object Reference") "None" true (struct :`G` 0.094117 :`B` 1.0 :`A` 1.0))
  (set `self.ConeTraceOffset` _returnvalue_4)
  ;[1 1 1] cone trace
  ;;[1 1 1] Start at second iteration of spheres as first is already traced before
  (for _index (range 2 (+ (`self.ConeSteps`) 1))
    (bind _outhits (`KismetSystemLibrary.SphereTraceMulti` (`self.ConeTraceOffset`) _returnvalue_3 (* (`KismetMathLibrary.Conv_IntToDouble` _index) (`.Radius_60_961B55264A85427CF39F2E901AD90497` (break `/Game/Collab/Tech/Abilities/Refactor/S_AbilityStats` (`self.AbilityStats`)))) "TraceTypeQuery1" false (`|MakeArray` self :!type "Actor Object Reference")))
    ;[1 1 1] set new offset to previous sphere trace point
    (set `self.ConeTraceOffset` _returnvalue_3)
    ;[1 1 1] damage actors hit
    (for _array_element _outhits
      (bind (_bblockinghit _binitialoverlap _time _distance _location _impactpoint _normal _impactnormal _physmat _hitactor) (`GameplayStatics.BreakHitResult` _array_element))
      (if (not (`KismetArrayLibrary.Array_Contains` (`self.ActorsAlreadyHit`) _hitactor))
        (`KismetArrayLibrary.Array_Add` (`self.ActorsAlreadyHit`) _hitactor)
        (if (`KismetMathLibrary.ClassIsChildOf` (`GameplayStatics.GetObjectClass` _hitactor) "/Game/Collab/Tech/AI/Pawns/BaseEnemyPawn.BaseEnemyPawn_C")
          (bind _iscrit_ (`self.IsCrit?` _hitactor))
          (if _iscrit_
            (message `/Game/Collab/Tech/Interfaces/CombatInterface.BeenCrit` _hitactor))
          (bind _damage (`self.CalculateDamage` _iscrit_))
          (`GameplayStatics.ApplyDamage` _hitactor _damage null (`self.PlayerRef`))))))
  ;;[1 1 1] finish ability and begin cooldown
  (`self.OnAbilityFinished` self))

(fn `UserConstructionScript`
  (`parent.UserConstructionScript`))