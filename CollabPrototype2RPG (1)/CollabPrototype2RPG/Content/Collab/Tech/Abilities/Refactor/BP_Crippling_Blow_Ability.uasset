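; Player melee ability Crippling Blow, which damages what is in front of the player and slows enemies.
; On use it plays a montage, waits until just before it ends, then box-traces forward for pawns, dynamic objects and destructibles.
; Non-enemy hits take damage directly, while enemies are deduplicated before receiving damage and a timed slow message.
; It then clears the hit list and signals that the ability has finished.
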(event `/Game/Collab/Tech/Abilities/Refactor/BPI_AbilityInteraction.Use`
  (bind _returnvalue (`GameplayStatics.GetPlayerCharacter` 0))
  (bind (_abilitystats_abilitytype _abilitystats_hitfx _abilitystats_cooldown _abilitystats_damage) (break `/Game/Collab/Tech/Abilities/Refactor/S_AbilityStats` (`self.AbilityStats`)))
  (bind _temphitactors (`self.TempHitActors`))
  (bind (_abilitystats_abilitytype_2 _abilitystats_hitfx_2 _abilitystats_cooldown_2 _abilitystats_damage_2) (break `/Game/Collab/Tech/Abilities/Refactor/S_AbilityStats` (`self.AbilityStats`)))
  (bind _returnvalue_2 (`self.K2_GetActorLocation` _returnvalue))
  (bind _returnvalue_3 (`Character.PlayAnimMontage` _returnvalue "/Game/Collab/Animation/AM_CripplingBlow.AM_CripplingBlow" 1.0 "None"))
  (`KismetSystemLibrary.Delay` (- _returnvalue_3 0.3))
  (bind _outhits (`KismetSystemLibrary.BoxTraceMultiForObjects` _returnvalue_2 (+ _returnvalue_2 (* (`self.GetActorForwardVector` (`GameplayStatics.GetPlayerCharacter` 0)) 100.0)) (80.0 80.0 80.0) (struct) (`|MakeArray` "ObjectTypeQuery3" "ObjectTypeQuery2" "ObjectTypeQuery6" :!type "EObjectTypeQuery Enum") false (`|MakeArray` (`GameplayStatics.GetPlayerCharacter` 0) :!type "Actor Object Reference") "None" true (struct :`R` 1.0 :`A` 1.0) (struct :`G` 1.0 :`A` 1.0) 0.5))
  (for _array_element _outhits
    (if (`KismetMathLibrary.ClassIsChildOf` (`GameplayStatics.GetObjectClass` (`.HitActor` (`GameplayStatics.BreakHitResult` _array_element))) "/Game/Collab/Tech/AI/Pawns/BaseEnemyPawn.BaseEnemyPawn_C")
      (`KismetArrayLibrary.Array_AddUnique` (`self.TempHitActors`) (`.HitActor` (`GameplayStatics.BreakHitResult` _array_element)))
      (else
        ;[1 1 1] if the actor isn't an enemy, apply damage (for destructibles)
        (`GameplayStatics.ApplyDamage` (`.HitActor` (`GameplayStatics.BreakHitResult` _array_element)) _abilitystats_damage_2 null (`GameplayStatics.GetPlayerCharacter` 0)))))
  (for _array_element_2 _temphitactors
    (`GameplayStatics.ApplyDamage` _array_element_2 _abilitystats_damage null (`GameplayStatics.GetPlayerCharacter` 0))
    (message `/Game/Collab/Tech/Interfaces/CombatInterface.Slow Effect` _array_element_2 0.5 7.5))
  (`KismetArrayLibrary.Array_Clear` _temphitactors)
  (`self.OnAbilityFinished` self))

(fn `UserConstructionScript`
  (`parent.UserConstructionScript`))