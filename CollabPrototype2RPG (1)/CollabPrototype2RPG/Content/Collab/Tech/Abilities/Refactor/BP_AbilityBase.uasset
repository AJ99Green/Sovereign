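; BP_AbilityBase is the base Blueprint for abilities such as Dash, Whirlwind and Fireball, identified by an AbilityIdentifier enum.
; The construction script scans DT_Abilities for the row whose AbilityType matches the identifier and stores it as AbilityStats.
; Use is a placeholder that prints the ability name and fires OnAbilityFinished, and Initialise is an empty stub.
; StartCooldown runs a one-shot timer from the stats' Cooldown, while CooldownFinished broadcasts OnCooldownFinished.
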(event `/Game/Collab/Tech/Abilities/Refactor/BPI_AbilityInteraction.Use`
  (`KismetSystemLibrary.PrintString` (`KismetStringLibrary.Concat_StrStr` (select `/Game/Collab/Tech/Abilities/Refactor/E_AbilityIdentifier` (`self.AbilityIdentifier`) :`NewEnumerator0` "Dash" :`NewEnumerator1` "Charge" :`NewEnumerator2` "Whirlwind" :`NewEnumerator3` "Flesh render" :`NewEnumerator4` "Crippling Blow" :`NewEnumerator5` "Fireball") " used!"))
  (`self.OnAbilityFinished` self))

(fn `CooldownFinished`
  (`self.OnCooldownFinished` self))

(fn `Initialise`)

(fn `StartCooldown`
  (bind (_abilitystats_abilitytype _abilitystats_hitfx _abilitystats_cooldown) (break `/Game/Collab/Tech/Abilities/Refactor/S_AbilityStats_Used` (`self.AbilityStats`)))
  (`KismetSystemLibrary.K2_SetTimerDelegate` (`|CreateDelegate` :!event `CooldownFinished`) _abilitystats_cooldown)
  (return))

(fn `UserConstructionScript`
  (bind _outrownames (`DataTableFunctionLibrary.GetDataTableRowNames` "/Game/Collab/Tech/Abilities/Refactor/DT_Abilities.DT_Abilities"))
  (for _array_element _outrownames
    (bind _returnvalue (`|GetDataTableRow` "/Game/Collab/Tech/Abilities/Refactor/DT_Abilities.DT_Abilities" _array_element)
      (:`then`
        (if (`|EnumEquality` (`.AbilityType_23_12A89D6D4F28B899771DC9BE49E3F350` (break `/Game/Collab/Tech/Abilities/Refactor/S_AbilityStats_Used` _returnvalue)) (`self.AbilityIdentifier`))
          (set `self.AbilityStats` _returnvalue))))))