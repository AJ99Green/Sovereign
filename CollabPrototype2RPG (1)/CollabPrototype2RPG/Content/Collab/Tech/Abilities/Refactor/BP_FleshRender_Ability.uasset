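; Flesh Render ability that deals damage in a cone from the player toward the cursor.
; On use it turns the character to the cached cursor hit point, plays a sword cast montage and waits half its length.
; The cone is approximated by chained multi-sphere traces with linearly widening radii, debug-drawn.
; Each newly hit actor after the initial trace takes damage once, then the ability signals it has finished.
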(event `/Game/Collab/Tech/Abilities/Refactor/BPI_AbilityInteraction.Use`
  (bind _returnvalue (`GameplayStatics.GetPlayerCharacter` 0))
  (bind (_abilitystats_abilitytype _abilitystats_hitfx _abilitystats_cooldown _abilitystats_damage) (break `/Game/Collab/Tech/Abilities/Refactor/S_AbilityStats` (`self.AbilityStats`)))
  (bind _conetraceoffset (`self.ConeTraceOffset`))
  (bind (_returnvalue_roll _returnvalue_pitch) (`KismetMathLibrary.BreakRotator` (`self.K2_GetActorRotation` _returnvalue)))
  (bind _returnvalue_2 (`self.K2_GetActorLocation` (`GameplayStatics.GetPlayerCharacter` 0)))
  (bind _returnvalue_3 (/ 1.0 (`KismetMathLibrary.Conv_IntToDouble` (`self.ConeSteps`))))
  (bind (_returnvalue_roll_2 _returnvalue_pitch_2 _returnvalue_yaw) (`KismetMathLibrary.BreakRotator` (`KismetMathLibrary.FindLookAtRotation` (`self.K2_GetActorLocation` _returnvalue) (`self.CachedCursorPos`))))
  (bind _returnvalue_4 (`KismetMathLibrary.GetDirectionUnitVector` _returnvalue_2 (`self.CachedCursorPos`)))
  (bind _returnvalue_5 (+ (* _returnvalue_4 (* 500.0 _returnvalue_3)) _conetraceoffset))
  (bind _returnvalue_6 (+ (* _returnvalue_4 (* 500.0 (/ 1.0 (`KismetMathLibrary.Conv_IntToDouble` (`self.ConeSteps`))))) _returnvalue_2))
  ;[1 1 1] cache hit cursor result for direction of cone trace
  (set `self.CachedCursorPos` (`.Location` (`GameplayStatics.BreakHitResult` (`PlayerController.GetHitResultUnderCursorByChannel` (`GameplayStatics.GetPlayerController` 0) "TraceTypeQuery1" true))))
  ;[1 1 1] set actor rotation to the direction we're using the ability in
  (`self.K2_SetActorRotation` _returnvalue (`KismetMathLibrary.MakeRotator` _returnvalue_roll _returnvalue_pitch _returnvalue_yaw) false)
  ;[1 1 1] play cast montage
  (bind _astop_down_character (cast `/Game/Collab/Tech/Character/TopDownCharacter` (`GameplayStatics.GetPlayerPawn` 0)))
  (bind _returnvalue_7 (`Character.PlayAnimMontage` _astop_down_character "/Game/Collab/Animation/Montage_CastSword.Montage_CastSword" 1.0 "None"))
  (`KismetSystemLibrary.Delay` (- _returnvalue_7 (/ _returnvalue_7 2.0)))
  ;[1 1 1] initial sphere trace
  (`KismetSystemLibrary.SphereTraceMulti` (`self.K2_GetActorLocation` (`GameplayStatics.GetPlayerCharacter` 0)) _returnvalue_6 (`self.StartRadius`) "TraceTypeQuery1" false (`|MakeArray` self :!type "Actor Object Reference") "ForDuration" true (struct :`G` 0.094117 :`B` 1.0 :`A` 1.0))
  (set `self.ConeTraceOffset` _returnvalue_6)
  ;[1 1 1] cone trace
  ;;[1 1 1] Start at second iteration of spheres as first is already traced before
  (for _index (range 2 (+ (`self.ConeSteps`) 1))
    (bind _outhits (`KismetSystemLibrary.SphereTraceMulti` _conetraceoffset _returnvalue_5 (`KismetMathLibrary.MapRangeClamped` (* _index _returnvalue_3) 0.0 1.0 (`self.StartRadius`) (`self.EndRadius`)) "TraceTypeQuery1" false (`|MakeArray` self :!type "Actor Object Reference") "ForDuration"))
    ;[1 1 1] set new offset to previous sphere trace point
    (set `self.ConeTraceOffset` _returnvalue_5)
    ;[1 1 1] damage actors hit
    (for _array_element _outhits
      (bind (_bblockinghit _binitialoverlap _time _distance _location _impactpoint _normal _impactnormal _physmat _hitactor) (`GameplayStatics.BreakHitResult` _array_element))
      (if (not (`KismetArrayLibrary.Array_Contains` (`self.ActorsAlreadyHit`) _hitactor))
        (`KismetArrayLibrary.Array_Add` (`self.ActorsAlreadyHit`) _hitactor)
        (`GameplayStatics.ApplyDamage` _hitactor _abilitystats_damage null (`GameplayStatics.GetPlayerCharacter` 0)))))
  ;[1 1 1] finish ability and begin cooldown
  (`self.OnAbilityFinished` self))

(fn `UserConstructionScript`
  (`parent.UserConstructionScript`))