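; Charge ability that teleports the player character a fixed distance toward the cursor, then damages actors around the landing point.
; The destination is projected onto the navmesh, falling back to a walkable point sampled along the line if within range.
; A sphere overlap captures actors on arrival; after the ability's duration they take damage, a hit effect spawns and the ability reports finished.
; Debug lines and spheres visualise each step.
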(event `/Game/Collab/Tech/Abilities/Refactor/BPI_AbilityInteraction.Use`
  (bind _returnvalue (`GameplayStatics.GetPlayerCharacter` 0))
  (bind _returnvalue_2 (`GameplayStatics.GetPlayerCharacter` 0))
  (bind (_abilitystats_abilitytype _abilitystats_hitfx _abilitystats_cooldown _abilitystats_damage _abilitystats_damageradius _abilitystats_slowamount _abilitystats_abilityduration) (break `/Game/Collab/Tech/Abilities/Refactor/S_AbilityStats_Used` (`self.AbilityStats`)))
  (bind (_abilitystats_abilitytype_2 _abilitystats_hitfx_2 _abilitystats_cooldown_2 _abilitystats_damage_2 _abilitystats_damageradius_2 _abilitystats_slowamount_2 _abilitystats_abilityduration_2) (break `/Game/Collab/Tech/Abilities/Refactor/S_AbilityStats_Used` (`self.AbilityStats`)))
  (bind _returnvalue_3 (`self.K2_GetActorLocation` _returnvalue_2))
  (bind _returnvalue_4 (`self.K2_GetActorLocation` _returnvalue))
  (bind _returnvalue_5 (`self.K2_GetActorLocation` (`GameplayStatics.GetPlayerCharacter` 0)))
  (bind _returnvalue_6 (+ (* (`KismetMathLibrary.GetDirectionUnitVector` _returnvalue_5 (`.Location` (`GameplayStatics.BreakHitResult` (`PlayerController.GetHitResultUnderCursorByChannel` (`GameplayStatics.GetPlayerController` 0) "TraceTypeQuery1" true)))) 500.0) _returnvalue_5))
  (bind _projectedlocation (`/Game/Collab/Tech/Character/BP_NavigationUtilities.FindWalkablePointAlongLine` _returnvalue_5 _returnvalue_6 20 self))
  (bind (_projectedlocation_2 _returnvalue_7) (`NavigationSystemV1.K2_ProjectPointToNavigation` _returnvalue_6 null null (1000.0 1000.0 1000.0)))
  (`KismetSystemLibrary.DrawDebugLine` _returnvalue_5 _returnvalue_6 (struct :`R` 1.0 :`B` 0.04282 :`A` 1.0) 1.0)
  ;[1 1 1] if on navmesh dont do rest
  (if _returnvalue_7
    (`KismetSystemLibrary.DrawDebugSphere` _projectedlocation_2 100.0 12 (struct :`G` 0.140468 :`B` 1.0 :`A` 1.0) 1.0)
    (`self.K2_SetActorLocation` _returnvalue _projectedlocation_2 false true)
    (bind _outactors (`KismetSystemLibrary.SphereOverlapActors` _returnvalue_4 250.0 (`|MakeArray` "ObjectTypeQuery3" "ObjectTypeQuery2" "ObjectTypeQuery1" :!type "EObjectTypeQuery Enum") null (`|MakeArray` (`GameplayStatics.GetPlayerCharacter` 0) :!type "Actor Object Reference")))
    (`KismetSystemLibrary.DrawDebugSphere` _returnvalue_4 250.0 12 (struct :`G` 1.0 :`B` 0.415794 :`A` 1.0) 1.0)
    (`KismetSystemLibrary.Delay` _abilitystats_abilityduration_2)
    (`self.ApplyDamageToArray` _outactors _returnvalue_4)
    (`self.OnAbilityFinished` self :!label _label)
    (elif (<= (`KismetMathLibrary.Vector_Distance` _returnvalue_5 _projectedlocation) 500.0)
      (`KismetSystemLibrary.DrawDebugSphere` _projectedlocation 100.0 12 (struct :`G` 0.140468 :`B` 1.0 :`A` 1.0) 1.0)
      (`self.K2_SetActorLocation` (`GameplayStatics.GetPlayerCharacter` 0) _projectedlocation false true)
      (bind _outactors_2 (`KismetSystemLibrary.SphereOverlapActors` _returnvalue_3 250.0 (`|MakeArray` "ObjectTypeQuery3" "ObjectTypeQuery2" "ObjectTypeQuery1" :!type "EObjectTypeQuery Enum") null (`|MakeArray` _returnvalue_2 :!type "Actor Object Reference")))
      (`KismetSystemLibrary.DrawDebugSphere` _returnvalue_3 250.0 12 (struct :`G` 1.0 :`B` 0.415794 :`A` 1.0) 1.0)
      (`KismetSystemLibrary.Delay` _abilitystats_abilityduration)
      (`self.ApplyDamageToArray` _outactors_2 _returnvalue_3)
      (goto _label))))

(fn `ApplyDamageToArray`
  (params (Actors :type "Array of Actor Object Reference") (AttackerLocation :type "Vector Structure"))
  (bind (_abilitystats_abilitytype _abilitystats_hitfx _abilitystats_cooldown _abilitystats_damage) (break `/Game/Collab/Tech/Abilities/Refactor/S_AbilityStats_Used` (`self.AbilityStats`)))
  (for _array_element Actors
    (bind _returnvalue (`GameplayStatics.ApplyDamage` _array_element _abilitystats_damage null (`GameplayStatics.GetPlayerPawn` 0)))
    (`KismetSystemLibrary.PrintString` (`KismetStringLibrary.Conv_DoubleToString` _returnvalue)))
  (`GameplayStatics.SpawnEmitterAtLocation` _abilitystats_hitfx (- AttackerLocation (0.0 0.0 106.25))))

(fn `UserConstructionScript`
  (`parent.UserConstructionScript`))