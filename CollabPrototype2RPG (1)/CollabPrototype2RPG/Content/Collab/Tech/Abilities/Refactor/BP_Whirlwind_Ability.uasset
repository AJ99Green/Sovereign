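; Whirlwind player ability that spins the character and repeatedly damages nearby enemies for a set duration.
; Use plays the spin montage, attaches a particle effect to the player and starts a short looping timer for ApplyDamageInRadius.
; Each tick sphere-traces around the player and damages BaseEnemyPawn hits, using radius and damage from AbilityStats.
; After the ability duration it clears the timer, destroys the effect and broadcasts OnAbilityFinished.
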(event `ApplyDamageInRadius`
  (bind (_abilitystats_abilitytype _abilitystats_hitfx _abilitystats_cooldown _abilitystats_damage _abilitystats_damageradius) (break `/Game/Collab/Tech/Abilities/Refactor/S_AbilityStats_Used` (`self.AbilityStats`)))
  (bind _returnvalue (`self.K2_GetActorLocation` (`GameplayStatics.GetPlayerCharacter` 0)))
  ;[1 1 1] sphere cast & apply damage
  (bind _outhits (`KismetSystemLibrary.SphereTraceMultiForObjects` :`Start` _returnvalue :`End` _returnvalue :`Radius` _abilitystats_damageradius :`ObjectTypes` (`|MakeArray` "ObjectTypeQuery2" "ObjectTypeQuery3" :!type "EObjectTypeQuery Enum") :`DrawTime` 1.0))
  (for _array_element _outhits
    (if (`KismetMathLibrary.ClassIsChildOf` (`GameplayStatics.GetObjectClass` (`.HitActor` (`GameplayStatics.BreakHitResult` _array_element))) "/Game/Collab/Tech/AI/Pawns/BaseEnemyPawn.BaseEnemyPawn_C")
      (`GameplayStatics.ApplyDamage` (`.HitActor` (`GameplayStatics.BreakHitResult` _array_element)) _abilitystats_damage null (`GameplayStatics.GetPlayerCharacter` 0)))))

(event `/Game/Collab/Tech/Abilities/Refactor/BPI_AbilityInteraction.Use`
  (bind _returnvalue (`GameplayStatics.GetPlayerPawn` 0))
  (bind (_abilitystats_abilitytype _abilitystats_hitfx) (break `/Game/Collab/Tech/Abilities/Refactor/S_AbilityStats_Used` (`self.AbilityStats`)))
  (bind (_abilitystats_abilitytype_2 _abilitystats_hitfx_2 _abilitystats_cooldown _abilitystats_damage _abilitystats_damageradius _abilitystats_slowamount _abilitystats_abilityduration) (break `/Game/Collab/Tech/Abilities/Refactor/S_AbilityStats_Used` (`self.AbilityStats`)))
  (bind _astop_down_character (cast `/Game/Collab/Tech/Character/TopDownCharacter` _returnvalue)
    (:`then`
      (`Character.PlayAnimMontage` _astop_down_character "/Game/Collab/Animation/Montage_Player_Spin.Montage_Player_Spin" 1.0 "None"))
    (:`CastFailed`
      _))
  (bind _returnvalue_2 (`GameplayStatics.SpawnEmitterAttached` _abilitystats_hitfx (`Actor.RootComponent` _returnvalue) "None" (0.0 0.0 0.0) (struct) (2.0 2.0 2.0) "SnapToTarget"))
  (bind _returnvalue_3 (`KismetSystemLibrary.K2_SetTimerDelegate` (delegate `ApplyDamageInRadius`) 0.2 true))
  (`KismetSystemLibrary.Delay` _abilitystats_abilityduration)
  (`KismetSystemLibrary.K2_ClearAndInvalidateTimerHandle` _returnvalue_3)
  (`ActorComponent.K2_DestroyComponent` _returnvalue_2)
  (`self.OnAbilityFinished` self))

(fn `UserConstructionScript`
  (`parent.UserConstructionScript`))