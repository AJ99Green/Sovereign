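; Blueprint function library of helpers for ability stats, covering lookup by ability type and display text.
; GetAbilityStatsByIdentifier linearly scans DT_Abilities rows and returns the first whose AbilityType matches.
; FormatAbilityStatsToString builds a summary of truncated cooldown, damage, radius, slow and duration, plus an Empty flag when all truncate to zero.
; GetAbilityNameFromStats supplies its name through a hardcoded Select on the ability type enum.
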(fn `Format Ability Stats to String`
  (params (AbilityStats :type "/Game/Collab/Tech/Abilities/Refactor/S_AbilityStats Structure"))
  (returns (FormattedStats :type Text) (bEmpty :type Boolean))
  (bind (_abilitytype _hitfx _cooldown _damage _radius _abilityduration _abilitythumbnail _skilltreeicon _abilitydemovideo _1hanimation _2hanimation _currentrage _maxrage _raging _slowpercentage) (break `/Game/Collab/Tech/Abilities/Refactor/S_AbilityStats` AbilityStats))
  (bind _returnvalue (`KismetMathLibrary.FTrunc` _abilityduration))
  (bind _returnvalue_2 (`KismetMathLibrary.FTrunc` _damage))
  (bind _returnvalue_3 (`KismetMathLibrary.FTrunc` _radius))
  (bind _returnvalue_4 (`KismetMathLibrary.FTrunc` _slowpercentage))
  (bind _returnvalue_5 (`KismetMathLibrary.FTrunc` _cooldown))
  (return (`|FormatText` "{0} \nCooldown: {1} \nDamage: {2} \nDamage Radius: {3} \nSlow Amount: {4} \nCast Duration: {5}" (`self.Get Ability Name from Stats` AbilityStats) (`KismetStringLibrary.Conv_IntToString` _returnvalue_5) (`KismetStringLibrary.Conv_IntToString` _returnvalue_2) (`KismetStringLibrary.Conv_IntToString` _returnvalue_3) (`KismetStringLibrary.Conv_IntToString` _returnvalue_4) (`KismetStringLibrary.Conv_IntToString` _returnvalue)) (and (== _returnvalue_5 0) (== _returnvalue_2 0) (== _returnvalue_3 0) (== _returnvalue_4 0) (== _returnvalue 0))))

(fn `Get Ability Name from Stats`
  (params (AbilityStats :type "/Game/Collab/Tech/Abilities/Refactor/S_AbilityStats Structure"))
  (returns (`Ability Name` :type String))
  (return (select `/Game/Collab/Tech/Abilities/Refactor/E_AbilityIdentifier` (`.AbilityType_23_12A89D6D4F28B899771DC9BE49E3F350` (break `/Game/Collab/Tech/Abilities/Refactor/S_AbilityStats` AbilityStats)) :`NewEnumerator2` "Whirlwind" :`NewEnumerator4` "Crippling Blow" :`NewEnumerator1` "Charge" :`NewEnumerator7` "Rage" :`NewEnumerator6` "Fleshrender" :`NewEnumerator3` "Earthshaker" :`NewEnumerator8` "Stampede" :`NewEnumerator9` "Smite" :`NewEnumerator10` "Consecration" :`NewEnumerator11` "ImprovedConsecration" :`NewEnumerator12` "LayOnHands" :`NewEnumerator13` "CallTheHeavens" :`NewEnumerator14` "BlessTheEarth" :`NewEnumerator15` "Communion" :`NewEnumerator5` "Fireball")))

(fn `GetAbilityStatsByIdentifier`
  (params (AbilityIdentifier :type "/Game/Collab/Tech/Abilities/Refactor/E_AbilityIdentifier Enum" :default "NewEnumerator0"))
  (returns (OutputPin :type "/Game/Collab/Tech/Abilities/Refactor/S_AbilityStats Structure"))
  (bind _outrownames (`DataTableFunctionLibrary.GetDataTableRowNames` "/Game/Collab/Tech/Abilities/Refactor/DT_Abilities.DT_Abilities"))
  (for _array_element _outrownames
    (bind _returnvalue (`|GetDataTableRow` "/Game/Collab/Tech/Abilities/Refactor/DT_Abilities.DT_Abilities" _array_element)
      (:`then`
        (if (`|EnumEquality` (`.AbilityType_23_12A89D6D4F28B899771DC9BE49E3F350` (break `/Game/Collab/Tech/Abilities/Refactor/S_AbilityStats` _returnvalue)) AbilityIdentifier)
          (return _returnvalue))))))