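; BP_CallTheHeavens is a Paladin area-of-effect attack that only fires while the player stands in a consecration.
; Use polls the player's other abilities for an in-range check and resets this ability if none pass.
; On success it plays sound, montage and radius-scaled particles at the player's feet.
; After a short delay, a sphere trace deals Intellect-scaled, crit-capable damage to enemies, optionally applying burn, then the ability finishes.
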(event `/Game/Collab/Tech/Abilities/Refactor/BPI_AbilityInteraction.Use`
  (params (PlayerRef :type "/Game/Collab/Tech/Character/TopDownCharacter Object Reference"))
  ;[1 1 1] On Ability Used
  (bind _output_get (set `self.PlayerRef` PlayerRef))
  ;;[1 1 1] Check to see if in consecration, if in then do ability, if not in then reset ability as it cannot be used
  (for _array_element (`/Game/Collab/Tech/Abilities/Refactor/BPA_AbilityManager.PlayerAbilities` (`/Game/Collab/Tech/Character/TopDownCharacter.BPA_AbilityManager` _output_get))
    (bind _inrange_ (message `/Game/Collab/Tech/Abilities/Refactor/BPI_AbilityInteraction.InRangeCheck` (`.CurrentAbilityActor_11_35401D234724918569DEEA99193974EF` (break `/Game/Collab/Tech/Abilities/Refactor/S_AbilityData` _array_element))))
    (if _inrange_
      (set `self.InConsecration` true)
      (break)
      (else
        (set `self.InConsecration` false))))
  (if (`self.InConsecration`)
    (`self.CallTheHeavens`)
    (else
      (`/Game/Collab/Tech/Abilities/Refactor/BPA_AbilityManager.ResetAbility` (`/Game/Collab/Tech/Character/TopDownCharacter.BPA_AbilityManager` (`self.PlayerRef`)) (`GameplayStatics.GetObjectClass` self)))))

(event `CallTheHeavens`
  (bind _location (`self.Location`))
  (bind _playerref (`self.PlayerRef`))
  (bind ((`HitFX_3_A4D89F414F998065D4C18EB26A3183FF` _hitfx) (`Radius_60_961B55264A85427CF39F2E901AD90497` _radius)) (break `/Game/Collab/Tech/Abilities/Refactor/S_AbilityStats` (`self.AbilityStats`)))
  (bind (_returnvalue_x _returnvalue_y _returnvalue_z) (`KismetMathLibrary.BreakVector` (`self.K2_GetActorLocation` _playerref)))
  (bind _returnvalue (/ _radius 100.0))
  ;[1 1 1] Call the Heavens, AOE battack
  (`GameplayStatics.PlaySound2D` "/Game/Collab/Design/AbilitySFX/PaladinAbilitySFX/CallTheHeavens.CallTheHeavens" 1.0 1.0 0.0 null null)
  (`Character.PlayAnimMontage` (`self.PlayerRef`) (`.1HAnimation_64_B819E5424B8DBA9AD91893A57EC41E4A` (break `/Game/Collab/Tech/Abilities/Refactor/S_AbilityStats` (`self.AbilityStats`))) 1.0 "None")
  (bind _output_get (set `self.Location` (`KismetMathLibrary.MakeVector` _returnvalue_x _returnvalue_y (- _returnvalue_z (.z (`.BoxExtent` (`self.GetActorBounds` _playerref true false)))))))
  (bind _returnvalue_2 (`GameplayStatics.SpawnEmitterAtLocation` _hitfx _output_get (struct) (`KismetMathLibrary.MakeVector` _returnvalue _returnvalue _returnvalue)))
  (set `self.ParticleEffect` _returnvalue_2)
  (`KismetSystemLibrary.Delay` (* (`.AbilityDuration_19_E06109C245A749342E1A3BBC0C674573` (break `/Game/Collab/Tech/Abilities/Refactor/S_AbilityStats` (`self.AbilityStats`))) 0.2))
  (bind _outhits (`KismetSystemLibrary.SphereTraceMultiForObjects` :`Start` _location :`End` _location :`Radius` (`.Radius_60_961B55264A85427CF39F2E901AD90497` (break `/Game/Collab/Tech/Abilities/Refactor/S_AbilityStats` (`self.AbilityStats`))) :`ObjectTypes` (`|MakeArray` "ObjectTypeQuery2" "ObjectTypeQuery3" :!type "EObjectTypeQuery Enum") :`DrawTime` 1.0))
  (for _array_element _outhits
    (if (`KismetMathLibrary.ClassIsChildOf` (`GameplayStatics.GetObjectClass` (`.HitActor` (`GameplayStatics.BreakHitResult` _array_element))) "/Game/Collab/Tech/AI/Pawns/BaseEnemyPawn.BaseEnemyPawn_C")
      (bind _iscrit_ (`self.IsCrit?` (`.HitActor` (`GameplayStatics.BreakHitResult` _array_element))))
      (if _iscrit_
        (message `/Game/Collab/Tech/Interfaces/CombatInterface.BeenCrit` (`.HitActor` (`GameplayStatics.BreakHitResult` _array_element))))
      (bind _damage (`self.CalculateDamageWithIntellect` _iscrit_))
      (`GameplayStatics.ApplyDamage` (`.HitActor` (`GameplayStatics.BreakHitResult` _array_element)) _damage null (`self.PlayerRef`))
      (if (`self.Burn?`)
        (message `/Game/Collab/Tech/Interfaces/CombatInterface.Burn Effect` (`.HitActor` (`GameplayStatics.BreakHitResult` _array_element)) (`self.BurnTime`) (`self.BurnDamage`)))))
  (`KismetSystemLibrary.Delay` (* (`.AbilityDuration_19_E06109C245A749342E1A3BBC0C674573` (break `/Game/Collab/Tech/Abilities/Refactor/S_AbilityStats` (`self.AbilityStats`))) 0.8))
  (`ActorComponent.K2_DestroyComponent` (`self.ParticleEffect`))
  (`self.OnAbilityFinished` self))

(fn `UserConstructionScript`
  (`parent.UserConstructionScript`))