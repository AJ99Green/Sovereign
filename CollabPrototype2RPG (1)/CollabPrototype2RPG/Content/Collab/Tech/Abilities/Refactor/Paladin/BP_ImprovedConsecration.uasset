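; Paladin Improved Consecration ability that places a timed damage zone at the player's feet.
; A looping timer sphere-traces for enemies, dealing Intellect-scaled, crit-capable damage and healing the player for a fraction of it.
; A spawned sphere collider supports tracking whether the player is inside.
; Bless doubles damage; Commune ends the zone early to deal remaining ticks as one burst without healing, resetting the ability if Blessed.
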(event `/Game/Collab/Tech/Abilities/Refactor/BPI_AbilityInteraction.Use`
  (params (PlayerRef :type "/Game/Collab/Tech/Character/TopDownCharacter Object Reference"))
  (bind _playerref (`self.PlayerRef`))
  (bind ((`HitFX_3_A4D89F414F998065D4C18EB26A3183FF` _hitfx) (`Radius_60_961B55264A85427CF39F2E901AD90497` _radius)) (break `/Game/Collab/Tech/Abilities/Refactor/S_AbilityStats` (`self.AbilityStats`)))
  (bind (_returnvalue_x _returnvalue_y _returnvalue_z) (`KismetMathLibrary.BreakVector` (`self.K2_GetActorLocation` _playerref)))
  (bind _returnvalue (/ _radius 100.0))
  ;[1 1 1] On Improved Consecration used
  (bind _output_get (set `self.PlayerRef` PlayerRef))
  (`Character.PlayAnimMontage` _output_get (`.1HAnimation_64_B819E5424B8DBA9AD91893A57EC41E4A` (break `/Game/Collab/Tech/Abilities/Refactor/S_AbilityStats` (`self.AbilityStats`))) 1.0 "None")
  (bind _output_get_2 (set `self.Location` (`KismetMathLibrary.MakeVector` _returnvalue_x _returnvalue_y (- _returnvalue_z (.z (`.BoxExtent` (`self.GetActorBounds` _playerref true false)))))))
  (`self.ConsecrationSphereCollision` _output_get_2)
  (bind _returnvalue_2 (`GameplayStatics.SpawnEmitterAtLocation` _hitfx _output_get_2 (struct) (`KismetMathLibrary.MakeVector` _returnvalue _returnvalue _returnvalue)))
  (set `self.ParticleEffect` _returnvalue_2)
  (bind _returnvalue_3 (`KismetSystemLibrary.K2_SetTimerDelegate` (`|CreateDelegate` :!event `ApplyDamageInRadius`) 0.25 true))
  (set `self.DamageTimerHandle` _returnvalue_3)
  (bind _returnvalue_4 (`KismetSystemLibrary.K2_SetTimerDelegate` (delegate `EndAbility`) (`.AbilityDuration_19_E06109C245A749342E1A3BBC0C674573` (break `/Game/Collab/Tech/Abilities/Refactor/S_AbilityStats` (`self.AbilityStats`)))))
  (set `self.AbilityTimerHandle` _returnvalue_4))

(event `EndAbility`
  ;[1 1 1] On Improved Consecration used
  (`KismetSystemLibrary.K2_ClearAndInvalidateTimerHandle` (`self.DamageTimerHandle`))
  (`ActorComponent.K2_DestroyComponent` (`self.ParticleEffect`))
  (`self.OnAbilityFinished` self)
  (if (`self.Blessed?`)
    (set `self.Blessed?` false)))

(event `ApplyDamageInRadius`
  (bind _location (`self.Location`))
  ;[1 1 1] On Improved Consecration tick apply damage and heal for damage dealt
  (bind _outhits (`KismetSystemLibrary.SphereTraceMultiForObjects` :`Start` _location :`End` _location :`Radius` (`.Radius_60_961B55264A85427CF39F2E901AD90497` (break `/Game/Collab/Tech/Abilities/Refactor/S_AbilityStats` (`self.AbilityStats`))) :`ObjectTypes` (`|MakeArray` "ObjectTypeQuery2" "ObjectTypeQuery3" :!type "EObjectTypeQuery Enum") :`DrawTime` 1.0))
  (for _array_element _outhits
    (if (`KismetMathLibrary.ClassIsChildOf` (`GameplayStatics.GetObjectClass` (`.HitActor` (`GameplayStatics.BreakHitResult` _array_element))) "/Game/Collab/Tech/AI/Pawns/BaseEnemyPawn.BaseEnemyPawn_C")
      (bind _iscrit_ (`self.IsCrit?` (`.HitActor` (`GameplayStatics.BreakHitResult` _array_element))))
      (if _iscrit_
        (message `/Game/Collab/Tech/Interfaces/CombatInterface.BeenCrit` (`.HitActor` (`GameplayStatics.BreakHitResult` _array_element))))
      (bind _damage (`self.CalculateDamageWithIntellect` _iscrit_))
      ;;[1 1 1] If blessed deal double damage
      (if (`self.Blessed?`)
        (bind _returnvalue (* _damage 2.0))
        (`GameplayStatics.ApplyDamage` (`.HitActor` (`GameplayStatics.BreakHitResult` _array_element)) _returnvalue null (`self.PlayerRef`))
        (`/Game/Collab/Tech/Character/TopDownCharacter.ModifyHealth` (`self.PlayerRef`) (* _returnvalue 0.05) true)
        (else
          (`GameplayStatics.ApplyDamage` (`.HitActor` (`GameplayStatics.BreakHitResult` _array_element)) _damage null (`self.PlayerRef`))
          (`/Game/Collab/Tech/Character/TopDownCharacter.ModifyHealth` (`self.PlayerRef`) (* _damage 0.05) true))))))

(event `/Game/Collab/Tech/Abilities/Refactor/BPI_AbilityInteraction.Bless`
  ;[1 1 1] Blessed
  (set `self.Blessed?` true))

(event `/Game/Collab/Tech/Abilities/Refactor/BPI_AbilityInteraction.Commune`
  (params (CommuneFX :type "ParticleSystem Object Reference"))
  (bind _location (`self.Location`))
  (bind _particleeffect (`self.ParticleEffect`))
  (bind _returnvalue (/ (`.Radius_60_961B55264A85427CF39F2E901AD90497` (break `/Game/Collab/Tech/Abilities/Refactor/S_AbilityStats` (`self.AbilityStats`))) 200.0))
  ;[1 1 1] Commune, trigger remaining consecration instantly
  (set `self.RemainingTicks` (/ (`KismetSystemLibrary.K2_GetTimerRemainingTimeHandle` (`self.AbilityTimerHandle`)) 0.25))
  ;;[1 1 1] Stop Consecration
  (`KismetSystemLibrary.K2_ClearAndInvalidateTimerHandle` (`self.AbilityTimerHandle`))
  (`KismetSystemLibrary.K2_ClearAndInvalidateTimerHandle` (`self.DamageTimerHandle`))
  (`/Engine/EditorBlueprintResources/StandardMacros.IsValid` _particleeffect
    (:`Is Valid`
      (`ActorComponent.K2_DestroyComponent` _particleeffect)
      ;;[1 1 1] Spawn Communion Effect
      (`GameplayStatics.SpawnEmitterAtLocation` CommuneFX (`self.Location`) (struct) (`KismetMathLibrary.MakeVector` _returnvalue _returnvalue _returnvalue))
      (bind _outhits (`KismetSystemLibrary.SphereTraceMultiForObjects` :`Start` _location :`End` _location :`Radius` (`.Radius_60_961B55264A85427CF39F2E901AD90497` (break `/Game/Collab/Tech/Abilities/Refactor/S_AbilityStats` (`self.AbilityStats`))) :`ObjectTypes` (`|MakeArray` "ObjectTypeQuery2" "ObjectTypeQuery3" :!type "EObjectTypeQuery Enum") :`DrawTime` 1.0))
      (for _array_element _outhits
        (if (`KismetMathLibrary.ClassIsChildOf` (`GameplayStatics.GetObjectClass` (`.HitActor` (`GameplayStatics.BreakHitResult` _array_element))) "/Game/Collab/Tech/AI/Pawns/BaseEnemyPawn.BaseEnemyPawn_C")
          (bind _iscrit_ (`self.IsCrit?` (`.HitActor` (`GameplayStatics.BreakHitResult` _array_element))))
          (if _iscrit_
            (message `/Game/Collab/Tech/Interfaces/CombatInterface.BeenCrit` (`.HitActor` (`GameplayStatics.BreakHitResult` _array_element))))
          (bind _damage (`self.CalculateDamageWithIntellect` _iscrit_))
          (if (`self.Blessed?`)
            (`GameplayStatics.ApplyDamage` (`.HitActor` (`GameplayStatics.BreakHitResult` _array_element)) (* (* _damage 2.0) (`self.RemainingTicks`)) null (`self.PlayerRef`))
            (else
              (`GameplayStatics.ApplyDamage` (`.HitActor` (`GameplayStatics.BreakHitResult` _array_element)) (* _damage (`self.RemainingTicks`)) null (`self.PlayerRef`))))))
      (if (`self.Blessed?`)
        (set `self.Blessed?` false)
        (`/Game/Collab/Tech/Abilities/Refactor/BPA_AbilityManager.ResetAbility` (`/Game/Collab/Tech/Character/TopDownCharacter.BPA_AbilityManager` (`self.PlayerRef`)) (`GameplayStatics.GetObjectClass` self))))))

(fn `ConsecrationSphereCollision`
  (params (`Spawn Transform Location` :type "Vector Structure"))
  (bind _returnvalue (`|SpawnActorFromClass` "/Game/Collab/Tech/Abilities/Refactor/Paladin/BP_SphereCollider.BP_SphereCollider_C" (`KismetMathLibrary.MakeTransform` `Spawn Transform Location`) "Undefined" "OverrideRootScale" null null))
  (bind _output_get (set `self.SphereCollider` _returnvalue))
  (add `/Game/Collab/Tech/Abilities/Refactor/Paladin/BP_SphereCollider.PlayerCollideConsecration` (`self.SphereCollider`) (`|CreateDelegate` :!event `UpdatePlayerInConsecration`))
  (`/Game/Collab/Tech/Abilities/Refactor/Paladin/BP_SphereCollider.Init` _output_get (`.Radius_60_961B55264A85427CF39F2E901AD90497` (break `/Game/Collab/Tech/Abilities/Refactor/S_AbilityStats` (`self.AbilityStats`))) (`self.PlayerRef`)))

(fn `InRangeCheck`
  (returns (`InRange?` :type Boolean))
  (return (`self.PlayerInRange?`)))

(fn `UpdatePlayerInConsecration`
  (params (`PlayerInRange?` :type Boolean))
  (set `self.PlayerInRange?` `PlayerInRange?`))

(fn `UserConstructionScript`
  (`parent.UserConstructionScript`))