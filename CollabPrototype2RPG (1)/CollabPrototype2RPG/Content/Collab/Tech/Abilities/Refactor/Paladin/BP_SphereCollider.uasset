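; Sphere trigger actor for the Paladin's Consecration ability that reports whether a given player is inside its area.
; Init sets the sphere radius, stores the player reference and scans existing TopDownCharacter overlaps, so a player already inside is reported immediately.
; Begin and end overlap events filter for that player and call PlayerCollideConsecration with true on entry and false on exit.
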(event `Init`
  (params (InSphereRadius :type "Float (double-precision)") (PlayerRef :type "/Game/Collab/Tech/Character/TopDownCharacter Object Reference"))
  (`SphereComponent.SetSphereRadius` (`self.Sphere`) InSphereRadius true)
  (set `self.PlayerRef` PlayerRef)
  (for _array_element (`PrimitiveComponent.GetOverlappingActors` (`self.Sphere`) "/Game/Collab/Tech/Character/TopDownCharacter.TopDownCharacter_C")
    (if (== _array_element (`self.PlayerRef`))
      (`self.PlayerCollideConsecration` true)
      (break))))

(event `self.Sphere.OnComponentBeginOverlap`
  (params (OverlappedComponent :type "PrimitiveComponent Object Reference") (OtherActor :type "Actor Object Reference") (OtherComp :type "PrimitiveComponent Object Reference") (OtherBodyIndex :type Integer) (bFromSweep :type Boolean) (SweepResult :type "HitResult Structure (by ref)"))
  (if (== OtherActor (`self.PlayerRef`))
    (`self.PlayerCollideConsecration` true)))

(event `self.Sphere.OnComponentEndOverlap`
  (params (OverlappedComponent :type "PrimitiveComponent Object Reference") (OtherActor :type "Actor Object Reference") (OtherComp :type "PrimitiveComponent Object Reference") (OtherBodyIndex :type Integer))
  (if (== OtherActor (`self.PlayerRef`))
    (`self.PlayerCollideConsecration` false)))

(fn `UserConstructionScript`)