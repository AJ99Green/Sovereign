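; BP_LayOnHands is a Paladin ability that heals its caster after a cast time.
; Use plays a sword-cast montage with an attached particle effect, waits for the ability duration, then swaps in a second effect.
; It calls ModifyHealth with current health divided by 0.5, so the heal amount is twice current health.
; After a brief delay it signals ability completion and destroys the effect.
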(event `/Game/Collab/Tech/Abilities/Refactor/BPI_AbilityInteraction.Use`
  (params (PlayerRef :type "/Game/Collab/Tech/Character/TopDownCharacter Object Reference"))
  ;[1 1 1] On Lay On Hands Cast
  (bind _output_get (set `self.PlayerRef` PlayerRef))
  (`Character.PlayAnimMontage` _output_get "/Game/Collab/Animation/Montage_CastSword.Montage_CastSword" 1.0 "None")
  (bind _returnvalue (`GameplayStatics.SpawnEmitterAttached` null (`Character.Mesh` (`self.PlayerRef`)) "None" (0.0 0.0 50.0) (struct) (2.0 2.0 2.0)))
  (set `self.ParticleEffect` _returnvalue)
  (`KismetSystemLibrary.Delay` (`.AbilityDuration_19_E06109C245A749342E1A3BBC0C674573` (break `/Game/Collab/Tech/Abilities/Refactor/S_AbilityStats` (`self.AbilityStats`))))
  (`ActorComponent.K2_DestroyComponent` (`self.ParticleEffect`))
  (bind _returnvalue_2 (`GameplayStatics.SpawnEmitterAttached` null (`Character.Mesh` (`self.PlayerRef`)) "None" (0.0 0.0 50.0) (struct) (2.0 2.0 2.0)))
  (set `self.ParticleEffect` _returnvalue_2)
  (`/Game/Collab/Tech/Character/TopDownCharacter.ModifyHealth` (`self.PlayerRef`) (/ (`.CurrentHealth_17_367AD4C44B1379799B82BABA9B631FE1` (break `/Game/Collab/Tech/Character/S_CharacterStats` (`/Game/Collab/Tech/Character/TopDownCharacter.CharacterStats` (`self.PlayerRef`)))) 0.5) true)
  (`KismetSystemLibrary.Delay` 0.2)
  (`self.OnAbilityFinished` self)
  (`ActorComponent.K2_DestroyComponent` (`self.ParticleEffect`)))

(fn `UserConstructionScript`
  (`parent.UserConstructionScript`))