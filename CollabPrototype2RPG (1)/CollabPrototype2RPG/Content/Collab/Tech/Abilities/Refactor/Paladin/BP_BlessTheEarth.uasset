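; Paladin ability Blueprint for Bless the Earth, which blesses Consecration to deal double damage according to its comments.
; On Use, it stores the player reference, plays the Bless sound and loops over the abilities in the player's ability manager.
; It sends BlessMessage to each ability's current actor, leaving the effect to the receiver, then immediately signals that the ability has finished.
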(event `/Game/Collab/Tech/Abilities/Refactor/BPI_AbilityInteraction.Use`
  (params (PlayerRef :type "/Game/Collab/Tech/Character/TopDownCharacter Object Reference"))
  ;[1 1 1] Bless consecration making is deal double damage
  (set `self.PlayerRef` PlayerRef)
  (`GameplayStatics.PlaySound2D` "/Game/Collab/Design/AbilitySFX/PaladinAbilitySFX/Bless.Bless" 1.0 1.0 0.0 null null)
  ;;[1 1 1] Bless consecration
  (for _array_element (`/Game/Collab/Tech/Abilities/Refactor/BPA_AbilityManager.PlayerAbilities` (`/Game/Collab/Tech/Character/TopDownCharacter.BPA_AbilityManager` (`self.PlayerRef`)))
    (message `/Game/Collab/Tech/Abilities/Refactor/BPI_AbilityInteraction.Bless` (`.CurrentAbilityActor_11_35401D234724918569DEEA99193974EF` (break `/Game/Collab/Tech/Abilities/Refactor/S_AbilityData` _array_element))))
  (`self.OnAbilityFinished` self))

(fn `UserConstructionScript`
  (`parent.UserConstructionScript`))