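; Base Blueprint for aimed abilities: Use starts a looping timer that moves a Niagara aim indicator until left click or a timeout.
; Each tick places the indicator MaxAimDistance from the player's feet toward the cursor hit, always at full range despite the "clamp" comment, with the beam ending at the feet.
; StopAim hides it, signals aim finish and passes its location to OnAimFinished, an empty hook.
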(event `StopAim`
  (bind _aimingns (`self.AimingNS`))
  (`KismetSystemLibrary.K2_ClearAndInvalidateTimerHandle` (`self.AimingHandle`))
  (`self.OnAbilityFinishAim` self)
  (`SceneComponent.SetVisibility` _aimingns false false)
  (`self.OnAimFinished` (`SceneComponent.K2_GetComponentLocation` _aimingns))
  (set `self.bAlreadyUsing` false))

(event `/Game/Collab/Tech/Abilities/Refactor/BPI_AbilityInteraction.Use`
  (if (not (`self.bAlreadyUsing`))
    (set `self.bAlreadyUsing` true)
    (`self.OnAbilityAim` self)
    (bind _returnvalue (`KismetSystemLibrary.K2_SetTimerDelegate` (delegate `AimAbility`) 0.01 true))
    (bind _output_get (set `self.AimingHandle` _returnvalue))
    (`KismetSystemLibrary.Delay` 5.0)
    (if (`KismetSystemLibrary.K2_IsTimerActiveHandle` _output_get)
      (`self.StopAim`))))

(event `AimAbility`
  (bind _returnvalue (`GameplayStatics.GetPlayerController` 0))
  (bind _returnvalue_2 (`GameplayStatics.GetPlayerPawn` 0))
  (bind (_returnvalue_x _returnvalue_y _returnvalue_z) (`KismetMathLibrary.BreakVector` (`self.K2_GetActorLocation` _returnvalue_2)))
  (bind _returnvalue_3 (`KismetMathLibrary.MakeVector` _returnvalue_x _returnvalue_y (- _returnvalue_z (.z (`.BoxExtent` (`self.GetActorBounds` _returnvalue_2 true false))))))
  (if (`PlayerController.IsInputKeyDown` _returnvalue "LeftMouseButton")
    (`self.StopAim`)
    (else
      (`SceneComponent.SetVisibility` (`self.AimingNS`) true false)
      (`SceneComponent.K2_SetWorldLocation` (`self.AimingNS`) (+ (* (`KismetMathLibrary.GetDirectionUnitVector` _returnvalue_3 (`.Location` (`GameplayStatics.BreakHitResult` (`PlayerController.GetHitResultUnderCursorByChannel` _returnvalue "TraceTypeQuery1" true)))) (`self.MaxAimDistance`)) _returnvalue_3) false false)
      (`FXSystemComponent.SetVectorParameter` (`self.AimingNS`) "User.BeamEndPosition" _returnvalue_3))))

(fn `OnAimFinished`
  (params (AimPosition :type "Vector Structure")))

(fn `UserConstructionScript`
  (`parent.UserConstructionScript`))