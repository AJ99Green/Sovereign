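; BP_Rage is an ability that toggles the warrior character's rage state on and off.
; On Use, it calls StopRaging if the warrior is already raging, otherwise Rage, then immediately signals that the ability has finished.
; The warrior reference is resolved lazily by casting player character 0 to CharacterWarrior and caching it; if that cast fails, nothing happens.
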(event `/Game/Collab/Tech/Abilities/Refactor/BPI_AbilityInteraction.Use`
  (`/Engine/EditorBlueprintResources/StandardMacros.IsValid` (`self.WarriorRef`)
    (:`Is Valid`
      _)
    (:`Is Not Valid`
      (bind _ascharacter_warrior (cast `/Game/Collab/Tech/Character/CharacterWarrior` (`GameplayStatics.GetPlayerCharacter` 0)))
      (set `self.WarriorRef` _ascharacter_warrior)))
  (if (`/Game/Collab/Tech/Character/CharacterWarrior.IsRaging` (`self.WarriorRef`))
    (`/Game/Collab/Tech/Character/CharacterWarrior.StopRaging` (`self.WarriorRef`))
    (else
      (`/Game/Collab/Tech/Character/CharacterWarrior.Rage` (`self.WarriorRef`))))
  (`self.OnAbilityFinished` self))

(fn `UserConstructionScript`
  (`parent.UserConstructionScript`))