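; Base ability Blueprint that provides shared stats, damage and cooldown logic for the game's abilities.
; Construction script copies the DT_Abilities row matching AbilityIdentifier into AbilityStats.
; Use stores the player, prints a debug message and broadcasts OnAbilityFinished; helpers roll Strength- or Intellect-scaled damage, with doubled crits likelier on bleeding targets.
; Initialise is empty, GetAnimation always returns the one-handed animation, and cooldowns use a timer and completion dispatcher.
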(event `/Game/Collab/Tech/Abilities/Refactor/BPI_AbilityInteraction.Use`
  (params (PlayerRef :type "/Game/Collab/Tech/Character/TopDownCharacter Object Reference"))
  (set `self.PlayerRef` PlayerRef)
  (`KismetSystemLibrary.PrintString` (`KismetStringLibrary.Concat_StrStr` (select `/Game/Collab/Tech/Abilities/Refactor/E_AbilityIdentifier` (`self.AbilityIdentifier`) :`NewEnumerator2` "Whirlwind" :`NewEnumerator4` "Crippling Blow" :`NewEnumerator1` "Charge" :`NewEnumerator7` "Rage" :`NewEnumerator6` "Fleshrender" :`NewEnumerator3` "Earthshaker" :`NewEnumerator8` "Stampede" :`NewEnumerator9` "Smite" :`NewEnumerator10` "Consecration" :`NewEnumerator11` "ImprovedConsecration" :`NewEnumerator12` "LayOnHands" :`NewEnumerator13` "CallTheHeavens" :`NewEnumerator14` "BlessTheEarth" :`NewEnumerator15` "Communion" :`NewEnumerator5` "Fireball") " used!"))
  (`self.OnAbilityFinished` self))

(fn `CalculateDamageWithIntellect`
  (params (`Crit?` :type Boolean))
  (returns (Damage :type "Float (double-precision)"))
  (bind _returnvalue (+ (`.Damage_9_F3F577364B193D803DFA64A17579BBCC` (break `/Game/Collab/Tech/Abilities/Refactor/S_AbilityStats` (`self.AbilityStats`))) (* (`KismetMathLibrary.Conv_IntToDouble` (`.Intellect_60_F75647844420E6E994254680D567A424` (break `/Game/Collab/Tech/Character/S_CharacterStats` (`/Game/Collab/Tech/Character/TopDownCharacter.CharacterStats` (`self.PlayerRef`))))) (`KismetMathLibrary.RandomFloatInRange` 0.18 0.22))))
  (if `Crit?`
    (return (* _returnvalue 2.0))
    (else
      (return _returnvalue))))

(fn `CalculateDamageWithStrength`
  (params (`Crit?` :type Boolean))
  (returns (Damage :type "Float (double-precision)"))
  (bind _returnvalue (+ (`.Damage_9_F3F577364B193D803DFA64A17579BBCC` (break `/Game/Collab/Tech/Abilities/Refactor/S_AbilityStats` (`self.AbilityStats`))) (* (`KismetMathLibrary.Conv_IntToDouble` (`.Strength_93_8F3DB7244A073A8BFCDF6AB4C9BB4C87` (break `/Game/Collab/Tech/Character/S_CharacterStats` (`/Game/Collab/Tech/Character/TopDownCharacter.CharacterStats` (`self.PlayerRef`))))) (`KismetMathLibrary.RandomFloatInRange` 0.18 0.22))))
  (if `Crit?`
    (return (* _returnvalue 2.0))
    (else
      (return _returnvalue))))

(fn `CooldownFinished`
  (`self.OnCooldownFinished` self))

(fn `GetAnimation`
  (returns (ReturnValue :type "AnimMontage Object Reference"))
  (bind ((`1HAnimation_64_B819E5424B8DBA9AD91893A57EC41E4A` _1hanimation) (`2HAnimation_63_8237E4F3499D1956C2F3BFBC963214D1` _2hanimation)) (break `/Game/Collab/Tech/Abilities/Refactor/S_AbilityStats` (`self.AbilityStats`)))
  (return (select `bool` false :`false` _1hanimation :`true` _2hanimation)))

(fn `Initialise`)

(fn `IsCrit?`
  (params (HitObject :type "Object Object Reference"))
  (returns (`IsCrit?` :type Boolean))
  (locals (CritChanceTemp :type "Float (double-precision)"))
  (bind ((`CritChance_82_529FBF964E30B1038D501BB8F7CAB51A` _critchance)) (break `/Game/Collab/Tech/Character/S_CharacterStats` (`/Game/Collab/Tech/Character/TopDownCharacter.CharacterStats` (`self.PlayerRef`))))
  (bind _is_bleeding (message `/Game/Collab/Tech/Interfaces/CombatInterface.IsBleeding` HitObject))
  (if _is_bleeding
    (set `local.CritChanceTemp` (+ _critchance 0.3))
    (else
      (set `local.CritChanceTemp` _critchance)))
  (return (`KismetMathLibrary.RandomBoolWithWeight` (`local.CritChanceTemp`))))

(fn `StartCooldown`
  (bind (_abilitystats_abilitytype _abilitystats_hitfx _abilitystats_cooldown) (break `/Game/Collab/Tech/Abilities/Refactor/S_AbilityStats` (`self.AbilityStats`)))
  (`KismetSystemLibrary.K2_SetTimerDelegate` (`|CreateDelegate` :!event `CooldownFinished`) _abilitystats_cooldown)
  (return))

(fn `UserConstructionScript`
  (bind _outrownames (`DataTableFunctionLibrary.GetDataTableRowNames` "/Game/Collab/Tech/Abilities/Refactor/DT_Abilities.DT_Abilities"))
  (for _array_element _outrownames
    (bind _returnvalue (`|GetDataTableRow` "/Game/Collab/Tech/Abilities/Refactor/DT_Abilities.DT_Abilities" _array_element)
      (:`then`
        (if (`|EnumEquality` (`.AbilityType_23_12A89D6D4F28B899771DC9BE49E3F350` (break `/Game/Collab/Tech/Abilities/Refactor/S_AbilityStats` _returnvalue)) (`self.AbilityIdentifier`))
          (set `self.AbilityStats` _returnvalue))))))