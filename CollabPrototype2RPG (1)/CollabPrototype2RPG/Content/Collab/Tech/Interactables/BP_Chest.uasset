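; BP_Chest is a one-time interactable chest that gives its contents to the player.
; On first interaction it spawns a pickup particle and sends each ChestContents item to the player pawn via PickupItemMessage.
; A Swing timeline feeds RInterpTo to rotate the lid open, then plays in reverse after ChestOpenTime.
; Cursor hover on MouseCollision toggles selection highlighting through BPAVisualSelection.
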(event `/Game/Collab/Tech/Interactables/BPI_Interact.Interact`
  (if (not (`self.Opened`))
    (`GameplayStatics.SpawnEmitterAttached` "/Game/InfinityBladeEffects/Effects/FX_Treasure/Loot/P_KeyPickup_01.P_KeyPickup_01" (`self.Chest`) "None" (0.0 0.0 0.0) (struct) (0.5 0.5 0.5))
    (set `self.Opened` true)
    (for _array_element (`self.chestContents`)
      (message `/Game/Collab/Tech/Interactables/BPI_PlayerInteraction.PickupItem` (`GameplayStatics.GetPlayerPawn` 0) _array_element))
    (`self.OpenChest`)
    (`KismetSystemLibrary.Delay` (`self.ChestOpenTime`))
    (`self.CloseChest`)))

(event `OpenChest`
  (bind (_direction _open) (`Timeline|Swing` :!via `PlayFromStart` :!label _label)
    (:`Update`
      (`SceneComponent.K2_SetRelativeRotation` (`self.ChestTop`) (`KismetMathLibrary.RInterpTo` (struct) (struct :`Roll` -140.0) _open 1.0) false false))))

(event `CloseChest`
  (goto _label :!via `ReverseFromEnd`))

(event `self.MouseCollision.OnBeginCursorOver`
  (params (TouchedComponent :type "PrimitiveComponent Object Reference"))
  (`/Game/Collab/Tech/SelectableObject/BPA_VisualSelection.Select` (`self.BPA_VisualSelection`) (`self.SelectColourValue`)))

(event `self.MouseCollision.OnEndCursorOver`
  (params (TouchedComponent :type "PrimitiveComponent Object Reference"))
  (`/Game/Collab/Tech/SelectableObject/BPA_VisualSelection.Deselect` (`self.BPA_VisualSelection`)))

(fn `UserConstructionScript`
  (`parent.UserConstructionScript`))