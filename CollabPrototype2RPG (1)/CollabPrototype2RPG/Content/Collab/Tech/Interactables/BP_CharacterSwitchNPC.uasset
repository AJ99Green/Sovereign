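; BP_CharacterSwitchNPC is an interactable NPC that swaps the player's character class with the one it holds.
; Overlap tracks the player in range, and cursor hover toggles a selection highlight.
; A click destroys the player and attached actors, spawns and possesses the stored class in place, then reinitializes the controller.
; The old class becomes the NPC's child actor, while a flag suppresses overlap detection during the swap.
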(event `self.MouseCollision.OnBeginCursorOver`
  (params (TouchedComponent :type "PrimitiveComponent Object Reference"))
  ;[1 1 1] Highlight
  (`/Game/Collab/Tech/SelectableObject/BPA_VisualSelection.Select` (`self.BPA_VisualSelection1`) (`self.SelectColourValue`)))

(event `self.InRangeCheck.OnComponentBeginOverlap`
  (params (OverlappedComponent :type "PrimitiveComponent Object Reference") (OtherActor :type "Actor Object Reference") (OtherComp :type "PrimitiveComponent Object Reference") (OtherBodyIndex :type Integer) (bFromSweep :type Boolean) (SweepResult :type "HitResult Structure (by ref)"))
  ;[1 1 1] Player is now in range of the chest
  (if (and (== OtherActor (`GameplayStatics.GetPlayerCharacter` 0)) (not (`self.PlayerSpawned`)))
    (set `self.InRange?` true)
    (bind _astop_down_character (cast `/Game/Collab/Tech/Character/TopDownCharacter` OtherActor))
    (set `self.PlayerRef` _astop_down_character)))

(event `self.MouseCollision.OnEndCursorOver`
  (params (TouchedComponent :type "PrimitiveComponent Object Reference"))
  ;[1 1 1] Highlight
  (`/Game/Collab/Tech/SelectableObject/BPA_VisualSelection.Deselect` (`self.BPA_VisualSelection1`)))

(event `self.InRangeCheck.OnComponentEndOverlap`
  (params (OverlappedComponent :type "PrimitiveComponent Object Reference") (OtherActor :type "Actor Object Reference") (OtherComp :type "PrimitiveComponent Object Reference") (OtherBodyIndex :type Integer))
  ;[1 1 1] Player is no longer in range of the chest
  (if (== OtherActor (`GameplayStatics.GetPlayerCharacter` 0))
    (set `self.InRange?` false)
    (set `self.PlayerRef` null)))

(event `self.MouseCollision.OnClicked`
  (params (TouchedComponent :type "PrimitiveComponent Object Reference") (ButtonPressed :type "Key Structure"))
  (bind _returnvalue (`GameplayStatics.GetPlayerController` 0))
  (bind _playerref (`self.PlayerRef`))
  ;[1 1 1] Character Switch
  (if (`KismetSystemLibrary.IsValid` (`self.PlayerRef`))
    (set `self.CharacterTransform` (`self.GetTransform` _playerref))
    (`Controller.UnPossess` (`GameplayStatics.GetPlayerController` 0))
    (set `self.NewCharacter` (`GameplayStatics.GetObjectClass` _playerref))
    (set `self.PlayerSpawned` true)
    (bind _output_get (set `self.DestroyChilderen` (`self.GetAttachedActors` _playerref true)))
    (for _array_element _output_get
      (`self.K2_DestroyActor` _array_element))
    (`self.K2_DestroyActor` (`self.PlayerRef`))
    (bind _returnvalue_2 (`|SpawnActorFromClass` (`self.Character`) (`self.CharacterTransform`) "AdjustIfPossibleButAlwaysSpawn" "OverrideRootScale" null null))
    (set `self.Character` (`self.NewCharacter`))
    (`self.SetCharacter`)
    (`Controller.Possess` _returnvalue _returnvalue_2)
    (bind _astop_down_controller (cast `/Game/Collab/Tech/Character/TopDownController` _returnvalue))
    (`/Game/Collab/Tech/Character/TopDownController.Init` _astop_down_controller)
    (set `self.PlayerRef` null)
    (set `self.PlayerSpawned` false)))

(fn `SetCharacter`
  (`ChildActorComponent.SetChildActorClass` (`self.CharacterChild`) (`self.Character`)))

(fn `UserConstructionScript`)