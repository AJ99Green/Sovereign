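; Blueprint library of inventory lookup helpers that read item definitions from the DT_InventoryItems data table.
; GetItemData treats the ID as a 1-based index into the table's row order, returning the row with a success flag or printing an error if not found.
; GetItemFromPrefab linearly scans every row and returns the first whose WorldActor matches the given prefab.
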(fn `Get Item Data`
  (params (ID :type Integer))
  (returns (`out ItemData` :type "/Game/Collab/Tech/Inventory/S_InventoryData Structure") (bSuccess :type Boolean))
  (bind _outrownames (`DataTableFunctionLibrary.GetDataTableRowNames` "/Game/Collab/Tech/Inventory/DT_InventoryItems.DT_InventoryItems"))
  (bind _returnvalue (`|GetDataTableRow` "/Game/Collab/Tech/Inventory/DT_InventoryItems.DT_InventoryItems" (`|GetArrayItem` _outrownames (- ID 1)))
    (:`then`
      (return _returnvalue true))
    (:`RowNotFound`
      (`KismetSystemLibrary.PrintString` null "Item not found (Check the ID)")
      (return (struct) false))))

(fn `Get Item From Prefab`
  (params (Prefab :type "/Game/Collab/Tech/Interactables/BP_InventoryItemOLD Class Reference"))
  (returns (`Out Row` :type "/Game/Collab/Tech/Inventory/S_InventoryData Structure"))
  (bind _outrownames (`DataTableFunctionLibrary.GetDataTableRowNames` "/Game/Collab/Tech/Inventory/DT_InventoryItems.DT_InventoryItems"))
  (for _array_element _outrownames
    (bind _returnvalue (`|GetDataTableRow` "/Game/Collab/Tech/Inventory/DT_InventoryItems.DT_InventoryItems" _array_element)
      (:`then`
        (if (== (`local.Prefab`) (`.WorldActor_52_B7B946EC49C9B7DB7F95279D4D2ABF75` (break `/Game/Collab/Tech/Inventory/S_InventoryData` _returnvalue)))
          (return _returnvalue))))))