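; BP_EntityInventory stores an entity's items as an array of ID and quantity entries, with functions to add, remove and query them.
; Adding stacks onto a matching ID or appends an entry, removing deletes entries that reach zero, and both fire inventory change notifications.
; GetItemData resolves IDs for the full data listing and search by type.
; FindInventoryItemByID is unfinished and returns no result.
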(event `/Game/Collab/Tech/Inventory/BPI_InventoryInteraction.AddItem`
  (params (ID :type Integer) (Quantity :type Integer))
  (`self.AddInventoryItem` ID Quantity))

(fn `AddInventoryItem`
  (params (ItemID :type Integer) (Amount :type Integer))
  (bind _itemid (`local.ItemID`))
  (bind _amount (`local.Amount`))
  (for (_array_element _array_index) (`self.Inventory Items`)
    (bind (_id _quantity) (break `/Game/Collab/Tech/Inventory/S_ComponentInventoryData` _array_element))
    (if (== _id (`local.ItemID`))
      (bind _returnvalue (+ _quantity (`local.Amount`)))
      (bind _structout (setmembers `/Game/Collab/Tech/Inventory/S_ComponentInventoryData` :`StructRef` _array_element :`Quantity` _returnvalue))
      (`KismetArrayLibrary.Array_Set` (`self.Inventory Items`) _array_index _structout)
      (`self.OnInventoryItemAdded` (`local.ItemID`) _returnvalue)
      (return)))
  ;[1 1 1] if item is not found, then add new entry to player inventory and add specified quantity
  (`KismetArrayLibrary.Array_Add` (`self.Inventory Items`) (make `/Game/Collab/Tech/Inventory/S_ComponentInventoryData` _itemid _amount))
  (`self.OnInventoryItemAdded` _itemid _amount)
  (return))

(fn `FindInventoryItemByID`
  (params (ID :type Integer))
  (if (`self.IsItemInInventory` ID)
    (for _array_element (`self.Inventory Items`)
      (if (== (`.ID_2_EED752D04F81CB5D59BAD2A1F19C6B81` (break `/Game/Collab/Tech/Inventory/S_ComponentInventoryData` _array_element)) (`local.ID`))
        _))))

(fn `FindInventoryItemByType`
  (params (ItemType :type "/Game/Collab/Tech/Inventory/E_ItemType Enum" :default "NewEnumerator0"))
  (returns (bSuccess :type Boolean) (ItemID :type Integer))
  (for _array_element (`self.Inventory Items`)
    (bind _id (break `/Game/Collab/Tech/Inventory/S_ComponentInventoryData` _array_element))
    (bind _out_itemdata (`/Game/Collab/Tech/Inventory/BP_InventoryLibrary.Get Item Data` _id))
    (if (`|EnumEquality` (`.ItemType_27_05B860D64E5522C80D5FF29BBABFDD3E` (break `/Game/Collab/Tech/Inventory/S_InventoryData` _out_itemdata)) (`local.ItemType`))
      (return true _id)))
  (return false -1))

(fn `GetFullInventoryData`
  (returns (Quantities :type "Array of Integer") (Data :type "Array of /Game/Collab/Tech/Inventory/S_InventoryData Structure"))
  (locals (`Local Quantity Data` :type "Array of Integer") (`Local Inv Data` :type "Array of /Game/Collab/Tech/Inventory/S_InventoryData Structure"))
  (for _array_element (`self.Inventory Items`)
    (bind (_id _quantity) (break `/Game/Collab/Tech/Inventory/S_ComponentInventoryData` _array_element))
    (bind (_out_itemdata _bsuccess) (`/Game/Collab/Tech/Inventory/BP_InventoryLibrary.Get Item Data` _id))
    (if _bsuccess
      (`KismetArrayLibrary.Array_Add` (`local.Local Quantity Data`) _quantity)
      (`KismetArrayLibrary.Array_Add` (`local.Local Inv Data`) _out_itemdata)))
  (return (`local.Local Quantity Data`) (`local.Local Inv Data`)))

(fn `IsItemInInventory`
  (params (ItemID :type Integer))
  (returns (bResult :type Boolean) (IndexOfItem :type Integer))
  (for (_array_element _array_index) (`self.Inventory Items`)
    (if (and (== (`.ID_2_EED752D04F81CB5D59BAD2A1F19C6B81` (break `/Game/Collab/Tech/Inventory/S_ComponentInventoryData` _array_element)) ItemID) true)
      (return true _array_index)))
  (return false -1))

(fn `RemoveInventoryItem`
  (params (ID :type Integer) (AmountToRemove :type Integer))
  (locals (Local_RemoveCount :type Integer))
  (bind (_bresult _indexofitem) (`self.IsItemInInventory` ID))
  (bind _output (`|GetArrayItem` (`self.Inventory Items`) _indexofitem))
  (bind _returnvalue (- (`.Quantity_4_C97275D044011C0AED0096ADAC4D06CC` (break `/Game/Collab/Tech/Inventory/S_ComponentInventoryData` _output)) (`local.AmountToRemove`)))
  (if _bresult
    (if (> _returnvalue 0)
      (bind _structout (setmembers `/Game/Collab/Tech/Inventory/S_ComponentInventoryData` :`StructRef` _output :`Quantity` _returnvalue))
      (`KismetArrayLibrary.Array_Set` (`self.Inventory Items`) _indexofitem _structout)
      (`self.OnInventoryItemRemoved` (`local.ID`) (`local.AmountToRemove`))
      (else
        (`KismetArrayLibrary.Array_RemoveItem` (`self.Inventory Items`) _output)
        (`self.OnInventoryItemRemoved` (`local.ID`) (`local.AmountToRemove`))))))