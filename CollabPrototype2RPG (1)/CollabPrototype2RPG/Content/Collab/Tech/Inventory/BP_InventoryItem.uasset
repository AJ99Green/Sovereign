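; A world pickup item that the player clicks to add to their inventory.
; Hovering the cursor highlights it through BPAVisualSelection and shows a tooltip widget initialised with the item ID on BeginPlay.
; An overlap range check gates clicks; a valid click sends ID and Quantity via BPI_InventoryInteraction to a component on the player pawn, then destroys the actor.
; Older overlap pickup, particle effect and popup widget logic remains but is disconnected.
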(event `self.ReceiveBeginPlay`
  (bind _aswb_item_tooltip (cast `/Game/Collab/Tech/Inventory/Widget/WB_ItemTooltip` (`WidgetComponent.GetUserWidgetObject` (`self.Widget`))))
  (`/Game/Collab/Tech/Inventory/Widget/WB_ItemTooltip.Init` _aswb_item_tooltip (`self.ID`)))

(event `self.InRangeCheck.OnComponentBeginOverlap`
  (params (OverlappedComponent :type "PrimitiveComponent Object Reference") (OtherActor :type "Actor Object Reference") (OtherComp :type "PrimitiveComponent Object Reference") (OtherBodyIndex :type Integer) (bFromSweep :type Boolean) (SweepResult :type "HitResult Structure (by ref)"))
  ;[1 1 1] Player is now in range of item
  (if (== OtherActor (`GameplayStatics.GetPlayerCharacter` 0))
    (set `self.InRange?` true)))

(event `self.MouseCollision.OnBeginCursorOver`
  (params (TouchedComponent :type "PrimitiveComponent Object Reference"))
  ;[1 1 1] Highlight
  (`/Game/Collab/Tech/SelectableObject/BPA_VisualSelection.Select` (`self.BPA_VisualSelection`) (`self.SelectColourValue`))
  (`SceneComponent.SetVisibility` (`self.Widget`) true false))

(event `self.MouseCollision.OnEndCursorOver`
  (params (TouchedComponent :type "PrimitiveComponent Object Reference"))
  ;[1 1 1] Highlight
  (`/Game/Collab/Tech/SelectableObject/BPA_VisualSelection.Deselect` (`self.BPA_VisualSelection`))
  (`SceneComponent.SetVisibility` (`self.Widget`) false false))

(event `self.InRangeCheck.OnComponentEndOverlap`
  (params (OverlappedComponent :type "PrimitiveComponent Object Reference") (OtherActor :type "Actor Object Reference") (OtherComp :type "PrimitiveComponent Object Reference") (OtherBodyIndex :type Integer))
  ;[1 1 1] Player is no longer in range of item
  (if (== OtherActor (`GameplayStatics.GetPlayerCharacter` 0))
    (set `self.InRange?` false)))

(event `self.MouseCollision.OnClicked`
  (params (TouchedComponent :type "PrimitiveComponent Object Reference") (ButtonPressed :type "Key Structure"))
  (bind _output (`|GetArrayItem` (`self.GetComponentsByInterface` (`GameplayStatics.GetPlayerPawn` 0) "/Game/Collab/Tech/Inventory/BPI_InventoryInteraction.BPI_InventoryInteraction_C")))
  ;[1 1 1] On clicked, if in range then pickup item
  (if (`self.InRange?`)
    (`/Engine/EditorBlueprintResources/StandardMacros.IsValid` _output
      (:`Is Valid`
        (message `/Game/Collab/Tech/Inventory/BPI_InventoryInteraction.AddItem` _output (`self.ID`) (`self.Quantity`))
        ;;[1 1 1] once picked up, destroy
        (`self.K2_DestroyActor`))
      (:`Is Not Valid`
        (`KismetSystemLibrary.PrintString` "---Inventory not found---" true true (struct :`R` 1.0 :`A` 1.0))))))

(event `self.MouseCollision.OnComponentBeginOverlap`
  (params (OverlappedComponent :type "PrimitiveComponent Object Reference") (OtherActor :type "Actor Object Reference") (OtherComp :type "PrimitiveComponent Object Reference") (OtherBodyIndex :type Integer) (bFromSweep :type Boolean) (SweepResult :type "HitResult Structure (by ref)"))
  ;[1 0.4041 0.3742] OLD
)

(event `self.ReceiveActorBeginCursorOver`
  ;[1 0.4041 0.3742] OLD
  ;;[1 1 1] contextual UMG handling
)

(event `self.ReceiveActorEndCursorOver`
  ;[1 0.4041 0.3742] OLD
  ;;[1 1 1] contextual UMG handling
)

(event `self.ReceiveDestroyed`
  ;[1 0.4041 0.3742] OLD
)

(fn `UserConstructionScript`)