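; Navigation utility Blueprint that finds a walkable point on the line between a pawn position and a target location.
; FindWalkablePointAlongLine samples evenly spaced points from the target back toward the pawn, projecting each onto the navmesh with a wide query extent.
; It stops at the first successful projection and returns that location, but reports success even if no sample projects.
; Debug line and sphere draws are left disconnected.
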(fn `FindWalkablePointAlongLine`
  (params (`Pawn Position` :type "Vector Structure") (`Target Location` :type "Vector Structure") (`Number Of Points Along Line` :type Integer) (Context :type "Actor Object Reference"))
  (returns (ProjectedLocation :type "Vector Structure") (bSuccess :type Boolean))
  (for _index (range (+ `Number Of Points Along Line` 1))
    (bind (_projectedlocation _returnvalue) (`NavigationSystemV1.K2_ProjectPointToNavigation` (`local.Context`) (- `Target Location` (* (`KismetMathLibrary.GetDirectionUnitVector` `Pawn Position` `Target Location`) (* _index (/ (`KismetMathLibrary.Vector_Distance` `Pawn Position` `Target Location`) (`KismetMathLibrary.Conv_IntToDouble` `Number Of Points Along Line`))))) null null (1000.0 1000.0 1000.0)))
    (if _returnvalue
      (break)))
  (return _projectedlocation true))