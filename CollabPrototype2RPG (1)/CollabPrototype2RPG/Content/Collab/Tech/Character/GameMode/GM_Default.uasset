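; Default game mode that spawns the player's character and forwards dialogue tree requests to a dialogue manager.
; BeginPlay destroys the auto-spawned character, then spawns and possesses a Warrior, initializes the TopDownController and stores its HUD.
; SpawnCharacter removes that HUD and spawns the selected Warrior or Paladin at a given transform through the same controller setup.
; A paused character-select widget flow is present but disconnected.
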(event `/Game/Collab/Tech/Character/GameMode/BPI_DialogueManagement.CloseDialogueTree`
  (`/Game/Collab/Tech/Character/GameMode/BPA_DialogueManager.CloseDialogue` (`self.BPA_DialogueManager`)))

(event `self.ReceiveBeginPlay`
  (bind _returnvalue (`GameplayStatics.GetPlayerController` 0))
  (bind _returnvalue_2 (`GameplayStatics.GetPlayerCharacter` 0))
  (`/Engine/EditorBlueprintResources/StandardMacros.IsValid` _returnvalue_2
    (:`Is Valid`
      ;[1 1 1] destroy initial character being spawned by gamemode
      (`self.K2_DestroyActor` _returnvalue_2))
    (:`Is Not Valid`
      _))
  (bind _returnvalue_3 (`|SpawnActorFromClass` "/Game/Collab/Tech/Character/WarriorCharacter.WarriorCharacter_C" (`self.SpawnPoint`) "Undefined" "OverrideRootScale" null null :!label _label))
  (`Controller.Possess` _returnvalue _returnvalue_3)
  (bind _astop_down_controller (cast `/Game/Collab/Tech/Character/TopDownController` _returnvalue :!label _label_2))
  (`/Game/Collab/Tech/Character/TopDownController.Init` _astop_down_controller)
  (set `self.HudRef` (`/Game/Collab/Tech/Character/TopDownController.HUDRef` _astop_down_controller)))

(event `SpawnCharacter`
  (params (Selection :type "/Game/Collab/Tech/Character/E_Characters Enum" :default "NewEnumerator0") (SpawnPoint :type "Transform Structure"))
  (bind _hudref (`self.HudRef`))
  (set `self.SpawnPoint` SpawnPoint)
  (`/Engine/EditorBlueprintResources/StandardMacros.IsValid` _hudref
    (:`Is Valid`
      (`Widget.RemoveFromParent` _hudref))
    (:`Is Not Valid`
      _))
  (switch `/Game/Collab/Tech/Character/E_Characters` Selection
    (:`NewEnumerator0`
      (goto _label))
    (:`NewEnumerator1`
      (bind _returnvalue (`|SpawnActorFromClass` "/Game/Collab/Tech/Character/PaladinCharacter.PaladinCharacter_C" (`self.SpawnPoint`) "Undefined" "OverrideRootScale" null null))
      (`Controller.Possess` (`GameplayStatics.GetPlayerController` 0) _returnvalue)
      (goto _label_2))))

(fn `StartDialogueTree`
  (params (DialogueTree :type "DataTable Object Reference"))
  (returns (DialogueWidget :type "/Game/Collab/Tech/UI/Dialogue/WB_PlayerDialogue Object Reference"))
  (bind _bpa_dialoguemanager (`self.BPA_DialogueManager`))
  (`/Game/Collab/Tech/Character/GameMode/BPA_DialogueManager.Open Dialogue Tree` _bpa_dialoguemanager DialogueTree)
  (bind _returnvalue (`/Game/Collab/Tech/Character/GameMode/BPA_DialogueManager.Start Dialogue Tree` _bpa_dialoguemanager))
  (return _returnvalue))

(fn `UserConstructionScript`)