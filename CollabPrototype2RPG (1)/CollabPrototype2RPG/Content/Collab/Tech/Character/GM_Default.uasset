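; Default game mode that opens play with a character selection screen and spawns the chosen hero.
; On BeginPlay it pauses the game, shows the WB_CharacterSelect widget and passes itself to that widget.
; Its SpawnCharacter event spawns a Warrior or Paladin at the supplied transform and has player controller 0 possess it.
; It then initializes that controller as a TopDownController.
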(event `self.ReceiveBeginPlay`
  (`GameplayStatics.SetGamePaused` true)
  (bind _returnvalue (`|CreateWidget` "/Game/Collab/Tech/Character/WB_CharacterSelect.WB_CharacterSelect_C"))
  (bind _output_get (set `self.CharacterSelectUI` _returnvalue))
  (`UserWidget.AddToViewport` _output_get 0)
  (`/Game/Collab/Tech/Character/WB_CharacterSelect.Init` _output_get self))

(event `SpawnCharacter`
  (params (Selection :type "/Game/Collab/Tech/Character/E_Characters Enum" :default "NewEnumerator0") (SpawnPoint :type "Transform Structure"))
  (bind _returnvalue (`GameplayStatics.GetPlayerController` 0))
  (set `self.SpawnPoint` SpawnPoint)
  (switch `/Game/Collab/Tech/Character/E_Characters` Selection
    (:`NewEnumerator0`
      (bind _returnvalue_2 (`|SpawnActorFromClass` "/Game/Collab/Tech/Character/WarriorCharacter.WarriorCharacter_C" (`self.SpawnPoint`) "Undefined" "OverrideRootScale" null null))
      (`Controller.Possess` _returnvalue _returnvalue_2))
    (:`NewEnumerator1`
      (bind _returnvalue_3 (`|SpawnActorFromClass` "/Game/Collab/Tech/Character/PaladinCharacter.PaladinCharacter_C" (`self.SpawnPoint`) "Undefined" "OverrideRootScale" null null))
      (`Controller.Possess` (`GameplayStatics.GetPlayerController` 0) _returnvalue_3)))
  (bind _astop_down_controller (cast `/Game/Collab/Tech/Character/TopDownController` _returnvalue))
  (`/Game/Collab/Tech/Character/TopDownController.Init` _astop_down_controller))

(fn `UserConstructionScript`)