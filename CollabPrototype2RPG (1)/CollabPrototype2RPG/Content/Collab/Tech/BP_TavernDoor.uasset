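; BP_TavernDoor is a clickable door that teleports the player to the spawn location of a connected door.
; Its collision overlap events set whether the player can interact, and hovering the cursor toggles selection feedback through BPAVisualSelection.
; A valid click plays a timeline that rotates the door mesh, then starts a camera fade from full opacity and moves the pawn, raised slightly above the destination point.
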(event `OpenDoor`
  (params (StartRotation :type "Rotator Structure"))
  (bind (_direction _newtrack_0) (`Timeline|MoveDoorTL`)
    (:`Update`
      (`SceneComponent.K2_SetRelativeRotation` (`self.SM_Door`) (`KismetMathLibrary.RLerp` StartRotation (struct :`Yaw` 15.0) _newtrack_0) false false))
    (:`Finished`
      (`PlayerCameraManager.StartCameraFade` :`self` (`GameplayStatics.GetPlayerCameraManager` 0) :`FromAlpha` 1.0 :`Duration` 2.0)
      (`self.K2_SetActorLocation` (`GameplayStatics.GetPlayerPawn` 0) (+ (`SceneComponent.K2_GetComponentLocation` (`/Game/Collab/Tech/BP_TavernDoor.SpawnLocation` (`self.ConnectingDoor`))) (0.0 0.0 96.0)) false false)
      (`KismetSystemLibrary.Delay` 2.0))))

(event `self.Interact`
  (`self.OpenDoor` (`SceneComponent.RelativeRotation` (`self.SM_Door`))))

(event `self.ReceiveActorBeginCursorOver`
  (`/Game/Collab/Tech/SelectableObject/BPA_VisualSelection.Select` (`self.BPA_VisualSelection`) 0))

(event `self.ReceiveActorEndCursorOver`
  (`/Game/Collab/Tech/SelectableObject/BPA_VisualSelection.Deselect` (`self.BPA_VisualSelection`)))

(event `self.InteractionDistCollision.OnComponentBeginOverlap`
  (params (OverlappedComponent :type "PrimitiveComponent Object Reference") (OtherActor :type "Actor Object Reference") (OtherComp :type "PrimitiveComponent Object Reference") (OtherBodyIndex :type Integer) (bFromSweep :type Boolean) (SweepResult :type "HitResult Structure (by ref)"))
  (if (== OtherActor (`GameplayStatics.GetPlayerPawn` 0))
    (set `self.bCanInteract` true)))

(event `self.InteractionDistCollision.OnComponentEndOverlap`
  (params (OverlappedComponent :type "PrimitiveComponent Object Reference") (OtherActor :type "Actor Object Reference") (OtherComp :type "PrimitiveComponent Object Reference") (OtherBodyIndex :type Integer))
  (if (== (stale `self.InteractionDistCollision.OnComponentBeginOverlap` OtherActor) (`GameplayStatics.GetPlayerPawn` 0))
    (set `self.bCanInteract` false)))

(event `self.mouseCollision.OnClicked`
  (params (TouchedComponent :type "PrimitiveComponent Object Reference") (ButtonPressed :type "Key Structure"))
  (if (`self.bCanInteract`)
    (`self.Interact`)))

(fn `UserConstructionScript`)